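; BP_CloudBase is a cloud actor that drifts along the world Y axis and removes itself on leaving a destroyer volume.
; BeginPlay picks a random speed between its min and max settings.
; Tick adds that speed to Y with a swept move, per frame without delta-time scaling.
; When its overlap with a BP_CloudDestroyer ends, the cloud destroys itself.
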(event `self.ReceiveBeginPlay`
  (set `self.FMoveSpeed` (`KismetMathLibrary.RandomFloatInRange` (`self.FCloudMinMoveSpeed`) (`self.FCloudMaxMoveSpeed`))))

(event `self.ReceiveActorEndOverlap`
  (params (OtherActor :type "Actor Object Reference"))
  (cast `/Game/Blueprints/Misc/BP_CloudDestroyer` OtherActor)
  (`self.K2_DestroyActor`))

(event `self.ReceiveTick`
  (params (DeltaSeconds :type "Float (single-precision)"))
  (bind (_returnvalue_x _returnvalue_y _returnvalue_z) (`KismetMathLibrary.BreakVector` (`self.K2_GetActorLocation`)))
  (`self.K2_SetActorLocation` (`KismetMathLibrary.MakeVector` _returnvalue_x (+ _returnvalue_y (`self.FMoveSpeed`)) _returnvalue_z) true))

(fn `UserConstructionScript`)