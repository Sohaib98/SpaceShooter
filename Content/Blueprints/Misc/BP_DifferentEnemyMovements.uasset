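; Spawner actor that lays out a lineup of BP_Enemy_Empty enemies, one for each of seven movement patterns.
; On BeginPlay it spawns them along +Y, starting at an offset from its own location and continuing at even intervals.
; Each spawn sets exactly one movement flag: three steps, top-to-bottom, bottom-to-top, up-and-down, top-to-center, bottom-to-center or random up-and-down.
; Only the first spawn inherits the spawner's rotation and scale.
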(event `self.ReceiveBeginPlay`
  (bind (_returnvalue_location _returnvalue_rotation _returnvalue_scale) (`KismetMathLibrary.BreakTransform` (`self.GetTransform`)))
  (bind _returnvalue (+ _returnvalue_location (0.0 5000.0 0.0)))
  (bind _returnvalue_2 (+ _returnvalue (0.0 1500.0 0.0)))
  (bind _returnvalue_3 (+ _returnvalue_2 (0.0 1500.0 0.0)))
  (bind _returnvalue_4 (+ _returnvalue_3 (0.0 1500.0 0.0)))
  (bind _returnvalue_5 (+ _returnvalue_4 (0.0 1500.0 0.0)))
  (bind _returnvalue_6 (+ _returnvalue_5 (0.0 1500.0 0.0)))
  (`|SpawnActorFromClass` "/Game/Blueprints/Enemies/BP_Enemy_Empty.BP_Enemy_Empty_C" (`KismetMathLibrary.MakeTransform` _returnvalue _returnvalue_rotation _returnvalue_scale) "Undefined" "OverrideRootScale" null true)
  (`|SpawnActorFromClass` "/Game/Blueprints/Enemies/BP_Enemy_Empty.BP_Enemy_Empty_C" (`KismetMathLibrary.MakeTransform` _returnvalue_2) "Undefined" "OverrideRootScale" null false true)
  (`|SpawnActorFromClass` "/Game/Blueprints/Enemies/BP_Enemy_Empty.BP_Enemy_Empty_C" (`KismetMathLibrary.MakeTransform` _returnvalue_3) "Undefined" "OverrideRootScale" null false false true)
  (`|SpawnActorFromClass` "/Game/Blueprints/Enemies/BP_Enemy_Empty.BP_Enemy_Empty_C" (`KismetMathLibrary.MakeTransform` _returnvalue_4) "Undefined" "OverrideRootScale" null false false false true)
  (`|SpawnActorFromClass` "/Game/Blueprints/Enemies/BP_Enemy_Empty.BP_Enemy_Empty_C" (`KismetMathLibrary.MakeTransform` _returnvalue_5) "Undefined" "OverrideRootScale" null false false false false true)
  (`|SpawnActorFromClass` "/Game/Blueprints/Enemies/BP_Enemy_Empty.BP_Enemy_Empty_C" (`KismetMathLibrary.MakeTransform` _returnvalue_6) "Undefined" "OverrideRootScale" null false false false false false true)
  (`|SpawnActorFromClass` "/Game/Blueprints/Enemies/BP_Enemy_Empty.BP_Enemy_Empty_C" (`KismetMathLibrary.MakeTransform` (+ _returnvalue_6 (0.0 1500.0 0.0))) "Undefined" "OverrideRootScale" null false false false false false false true))

(fn `UserConstructionScript`)