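; Cloud spawner actor that spawns one random cloud at BeginPlay, then keeps spawning more at a timed interval.
; Each spawn picks one of the first two CloudArray classes and gets its transform from GetRandomTransform, which combines random X, Z and uniform scale within variable bounds at a fixed far Y.
; Repeat timing comes from a Delay on Tick set by SpawnInterval, rather than a timer.
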(event `self.ReceiveBeginPlay`
  (bind _transform (`self.GetRandomTransform`))
  (`|SpawnActorFromClass` (`|GetArrayItem` (`self.CloudArray`) (`KismetMathLibrary.RandomInteger` 2)) _transform "Undefined" "OverrideRootScale"))

(event `self.ReceiveTick`
  (params (DeltaSeconds :type "Float (single-precision)"))
  (`KismetSystemLibrary.Delay` (`self.SpawnInterval`))
  (bind _transform (`self.GetRandomTransform`))
  (`|SpawnActorFromClass` (`|GetArrayItem` (`self.CloudArray`) (`KismetMathLibrary.RandomInteger` 2)) _transform "Undefined" "OverrideRootScale"))

(fn `GetRandomScale`
  (returns (RandomScale :type "Float (double-precision)"))
  (return (`KismetMathLibrary.RandomFloatInRange` (`self.FMinScale`) (`self.FMaxScale`))))

(fn `GetRandomTransform`
  (returns (Transform :type "Transform Structure"))
  (bind _randomx (`self.GetRandomX`))
  (bind _randomz (`self.GetRandomZ`))
  (bind _randomscale (`self.GetRandomScale`))
  (return (`KismetMathLibrary.MakeTransform` (`KismetMathLibrary.MakeVector` _randomx 30000.0 _randomz) (struct) (`KismetMathLibrary.Conv_DoubleToVector` _randomscale))))

(fn `GetRandomX`
  (returns (RandomX :type "Float (double-precision)"))
  (return (`KismetMathLibrary.RandomFloatInRange` (`self.FMinX`) (`self.FMaxX`))))

(fn `GetRandomZ`
  (returns (RandomZ :type "Float (double-precision)"))
  (return (`KismetMathLibrary.RandomFloatInRange` (`self.FMinZ`) (`self.FMaxZ`))))

(fn `UserConstructionScript`)