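; Enemy Blueprint that provides shoot and rotate functions, with no logic of its own calling them in this file.
; Shoot spawns a BpProjectileEnemyRocket at the world transform of the Scene1 component.
; The two rotate functions step the Cone's roll one degree either way, writing world roll into relative rotation and zeroing pitch and yaw.
; Tick and the construction script only call their parent versions.
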(event `self.ReceiveTick`
  (params (DeltaSeconds :type "Float (single-precision)"))
  (`parent.ReceiveTick` DeltaSeconds))

(fn `RotateClockWise`
  (bind _cone (`self.Cone`))
  (bind _returnvalue_roll (`KismetMathLibrary.BreakRotator` (`SceneComponent.K2_GetComponentRotation` _cone)))
  (`SceneComponent.K2_SetRelativeRotation` _cone (`KismetMathLibrary.MakeRotator` (+ _returnvalue_roll 1.0) 0.0) false false))

(fn `RotateCounterClockWise`
  (bind _cone (`self.Cone`))
  (bind _returnvalue_roll (`KismetMathLibrary.BreakRotator` (`SceneComponent.K2_GetComponentRotation` _cone)))
  (`SceneComponent.K2_SetRelativeRotation` _cone (`KismetMathLibrary.MakeRotator` (+ _returnvalue_roll -1.0) 0.0) false false))

(fn `Shoot`
  (`|SpawnActorFromClass` "/Game/Blueprints/Projectiles/bpProjectileEnemyRocket.bpProjectileEnemyRocket_C" (`SceneComponent.K2_GetComponentToWorld` (`self.Scene1`)) "Undefined" "OverrideRootScale"))

(fn `UserConstructionScript`
  (`parent.UserConstructionScript`))