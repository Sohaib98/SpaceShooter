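; Laser enemy Blueprint that periodically telegraphs and fires a laser projectile.
; Tick runs the parent logic, then chained latent Delays pace a repeating cycle: Charge about every ten seconds, with Shoot following a few seconds later.
; Charge plays a beam emitter offset along world Y from ProjectileSpawn; Shoot plays a muzzle emitter and spawns BpProjectileEnemyLaser3 there.
; The shot sound node is unconnected and never plays.
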(event `self.ReceiveBeginPlay`
  (`parent.ReceiveBeginPlay`))

(event `self.ReceiveTick`
  (params (DeltaSeconds :type "Float (single-precision)"))
  (`parent.ReceiveTick` DeltaSeconds)
  (`KismetSystemLibrary.Delay` 10.0)
  (`self.Charge`)
  (`KismetSystemLibrary.Delay` 4.0)
  (`self.Shoot`))

(fn `Charge`
  (bind (_returnvalue_x _returnvalue_y _returnvalue_z) (`KismetMathLibrary.BreakVector` (`SceneComponent.K2_GetComponentLocation` (`self.ProjectileSpawn`))))
  (`GameplayStatics.SpawnEmitterAtLocation` "/Game/ExampleContent/Effects/ParticleSystems/P_LaserBeamCharge.P_LaserBeamCharge" (`KismetMathLibrary.MakeVector` _returnvalue_x (+ _returnvalue_y -800.0) _returnvalue_z)))

(fn `Shoot`
  (bind _projectilespawn (`self.ProjectileSpawn`))
  (`GameplayStatics.SpawnEmitterAtLocation` "/Game/ExampleContent/Effects/ParticleSystems/P_LaserBeamShoot.P_LaserBeamShoot" (`SceneComponent.K2_GetComponentLocation` _projectilespawn))
  (`|SpawnActorFromClass` "/Game/Blueprints/Projectiles/bpProjectileEnemyLaser3.bpProjectileEnemyLaser3_C" (`SceneComponent.K2_GetComponentToWorld` _projectilespawn) "Undefined" "OverrideRootScale"))

(fn `UserConstructionScript`
  (`parent.UserConstructionScript`))