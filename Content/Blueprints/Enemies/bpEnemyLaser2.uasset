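; Laser enemy Blueprint that repeatedly fires BpProjectileEnemyLaser2 projectiles and defers to its parent for BeginPlay, Tick and construction.
; Tick feeds a Delay of FireRate, which ignores calls while pending and so acts as the repeating fire timer.
; Each completed delay spawns a projectile at the ProjectileSpawn transform and plays the EnemyShot sound at the world origin rather than at the enemy.
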(event `self.ReceiveBeginPlay`
  (`parent.ReceiveBeginPlay`))

(event `self.ReceiveTick`
  (params (DeltaSeconds :type "Float (single-precision)"))
  (`parent.ReceiveTick` DeltaSeconds)
  (`KismetSystemLibrary.Delay` (`self.FireRate`))
  (`|SpawnActorFromClass` "/Game/Blueprints/Projectiles/bpProjectileEnemyLaser2.bpProjectileEnemyLaser2_C" (`SceneComponent.K2_GetComponentToWorld` (`self.ProjectileSpawn`)) "Undefined" "OverrideRootScale")
  (`GameplayStatics.PlaySoundAtLocation` "/Game/Audio/EnemyShot.EnemyShot"))

(fn `UserConstructionScript`
  (`parent.UserConstructionScript`))