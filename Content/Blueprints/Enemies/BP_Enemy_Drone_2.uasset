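; Enemy drone that slows to a stop while firing tornado projectiles in a rotating pattern.
; Tick plays a timeline whose updates lerp ProjectileMovement velocity toward zero and feed a short Delay, which throttles calls to Shoot.
; Shoot spawns BP_ProjectileEnemy_Tornado at the drone's location and accumulates FRotation, stepping each shot's roll around to sweep the fire.
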(event `self.ReceiveTick`
  (params (DeltaSeconds :type "Float (single-precision)"))
  (bind _projectilemovement (`self.ProjectileMovement`))
  (bind (_direction _newtrack_0) (`Timeline|Timeline_1`)
    (:`Update`
      (set `MovementComponent.Velocity` (`KismetMathLibrary.VLerp` (`MovementComponent.Velocity` _projectilemovement) (0.0 0.0 0.0) _newtrack_0) _projectilemovement)
      (`KismetSystemLibrary.Delay` 0.2)
      (`self.Shoot` 10.0))))

(fn `Shoot`
  (params (Rotation :type "Float (double-precision)"))
  (bind _returnvalue (`self.GetTransform`))
  (bind _returnvalue_2 (+ Rotation (`self.FRotation`)))
  (`|SpawnActorFromClass` "/Game/Blueprints/Projectiles/BP_ProjectileEnemy_Tornado.BP_ProjectileEnemy_Tornado_C" (`KismetMathLibrary.MakeTransform` (.location _returnvalue) (`KismetMathLibrary.MakeRotator` _returnvalue_2 (.pitch (.rotation _returnvalue)) (.yaw (.rotation _returnvalue))) (.scale _returnvalue)) "Undefined" "OverrideRootScale" null 0.0 (0.0 -2000.0 0.0) (1.0 1.0 1.0))
  (set `self.FRotation` _returnvalue_2))

(fn `UserConstructionScript`
  (`parent.UserConstructionScript`))