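; Turret part for the modular combat drone enemy that fires continuously from two muzzles, with no targeting logic of its own.
; Tick runs into a Delay of the fire-rate variable, which acts as a repeating fire timer.
; Each cycle spawns a quarter-scale enemy projectile at both the right and left spawn points, using the turret's projectile speed and passing zero damage.
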(event `self.ReceiveTick`
  (params (DeltaSeconds :type "Float (single-precision)"))
  (`KismetSystemLibrary.Delay` (`self.FFireRate`))
  (`|SpawnActorFromClass` "/Game/Blueprints/Projectiles/BP_ProjectileEnemy.BP_ProjectileEnemy_C" (`SceneComponent.K2_GetComponentToWorld` (`self.ProjectileSpawnRight`)) "Undefined" "OverrideRootScale" null 0.0 (`self.VProjectileSpeed`) (0.25 0.25 0.25))
  (`|SpawnActorFromClass` "/Game/Blueprints/Projectiles/BP_ProjectileEnemy.BP_ProjectileEnemy_C" (`SceneComponent.K2_GetComponentToWorld` (`self.ProjectileSpawnLeft`)) "Undefined" "OverrideRootScale" null 0.0 (`self.VProjectileSpeed`) (0.25 0.25 0.25)))

(fn `UserConstructionScript`
  (`parent.UserConstructionScript`))