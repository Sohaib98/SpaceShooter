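; BP_Parts_GhostShip_LowerFrontSword is the lower front sword part of the modular GhostShip enemy, acting as a twin-muzzle gun.
; Tick feeds a Delay of FFireRate, which paces repeated volleys without a timer.
; Each volley spawns a BP_ProjectileEnemy at the right and left spawn points, sharing VProjectileSpeed but differing in scale, with Damage set to zero.
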(event `self.ReceiveTick`
  (params (DeltaSeconds :type "Float (single-precision)"))
  (`KismetSystemLibrary.Delay` (`self.FFireRate`))
  (`|SpawnActorFromClass` "/Game/Blueprints/Projectiles/BP_ProjectileEnemy.BP_ProjectileEnemy_C" (`SceneComponent.K2_GetComponentToWorld` (`self.ProjectileSpawnRight`)) "Undefined" "OverrideRootScale" null 0.0 (`self.VProjectileSpeed`) (0.5 0.5 0.5))
  (`|SpawnActorFromClass` "/Game/Blueprints/Projectiles/BP_ProjectileEnemy.BP_ProjectileEnemy_C" (`SceneComponent.K2_GetComponentToWorld` (`self.ProjectileSpawnLeft`)) "Undefined" "OverrideRootScale" null 0.0 (`self.VProjectileSpeed`) (1.0 2.0 1.0)))

(fn `UserConstructionScript`
  (`parent.UserConstructionScript`))