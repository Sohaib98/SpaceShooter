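; Ghost ship enemy Blueprint, from the modular ship enemies, that repeatedly fires a projectile.
; Tick runs through a Delay, so ShootFront fires roughly every two seconds.
; ShootFront spawns a stretched BP_ProjectileEnemy at the ProjectileSpawn transform with zero Damage passed in.
; Projectile Y speed is multiplied by EnemyMesh's world Y scale, so the mesh's scale sets both its magnitude and sign.
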(event `self.ReceiveTick`
  (params (DeltaSeconds :type "Float (single-precision)"))
  (`KismetSystemLibrary.Delay` 2.0)
  (`self.ShootFront`))

(fn `ShootFront`
  (bind (_returnvalue_x _returnvalue_y) (`KismetMathLibrary.BreakVector` (`SceneComponent.K2_GetComponentScale` (`self.EnemyMesh`))))
  (`|SpawnActorFromClass` "/Game/Blueprints/Projectiles/BP_ProjectileEnemy.BP_ProjectileEnemy_C" (`SceneComponent.K2_GetComponentToWorld` (`self.ProjectileSpawn`)) "Undefined" "OverrideRootScale" null 0.0 (`KismetMathLibrary.MakeVector` 0.0 (* _returnvalue_y 2000.0)) (2.0 1.0 1.0)))

(fn `UserConstructionScript`
  (`parent.UserConstructionScript`))