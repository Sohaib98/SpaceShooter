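; Enemy turret that fires a BP_ProjectileEnemy from its Scene component every tick while its Cone jitters back and forth in roll.
; A per-tick Timer counts down and wraps from -10 to 10, with its sign choosing one-degree clockwise or counter-clockwise steps.
; The clockwise phase runs slightly longer, so the wobble creeps round over time.
; Rotation and fire rate both depend on frame rate, as DeltaSeconds is unused.
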(event `self.ReceiveTick`
  (params (DeltaSeconds :type "Float (single-precision)"))
  (bind _timer (`self.Timer`))
  (`parent.ReceiveTick` DeltaSeconds)
  (if (>= (`self.Timer`) 0)
    (`self.RotateClockWise`)
    (`self.Shoot`)
    (set `self.Timer` (+ (`self.Timer`) -1))
    (else
      (`self.RotateCounterClockWise`)
      (`self.Shoot`)
      (set `self.Timer` (+ _timer -1))
      (if (<= _timer -10)
        (set `self.Timer` 10)))))

(fn `RotateClockWise`
  (bind _cone (`self.Cone`))
  (bind _returnvalue_roll (`KismetMathLibrary.BreakRotator` (`SceneComponent.K2_GetComponentRotation` _cone)))
  (`SceneComponent.K2_SetRelativeRotation` _cone (`KismetMathLibrary.MakeRotator` (+ _returnvalue_roll 1.0) 0.0) false false))

(fn `RotateCounterClockWise`
  (bind _cone (`self.Cone`))
  (bind _returnvalue_roll (`KismetMathLibrary.BreakRotator` (`SceneComponent.K2_GetComponentRotation` _cone)))
  (`SceneComponent.K2_SetRelativeRotation` _cone (`KismetMathLibrary.MakeRotator` (+ _returnvalue_roll -1.0) 0.0) false false))

(fn `Shoot`
  (`|SpawnActorFromClass` "/Game/Blueprints/Projectiles/BP_ProjectileEnemy.BP_ProjectileEnemy_C" (`SceneComponent.K2_GetComponentToWorld` (`self.Scene`)) "Undefined" "OverrideRootScale" null 0.0 (0.0 2222.0 0.0) (1.0 1.0 1.0)))

(fn `UserConstructionScript`
  (`parent.UserConstructionScript`))