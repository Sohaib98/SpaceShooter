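; Enemy drone variant that rolls its cone mesh while repeatedly firing enemy projectiles.
; Tick plays a looping timeline whose track drives both the target roll and the blend alpha of the cone's rotation.
; Timeline updates also feed a 0.2-second Delay, which throttles Shoot to spawn BpProjectileEnemy1 at the Scene component's transform with a fixed velocity along negative Y.
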(event `self.ReceiveTick`
  (params (DeltaSeconds :type "Float (single-precision)"))
  (bind _cone (`self.Cone`))
  (bind _returnvalue_roll (`KismetMathLibrary.BreakRotator` (`SceneComponent.K2_GetComponentRotation` _cone)))
  (bind (_direction _newtrack_0) (`Timeline|Timeline_1` :!label _label)
    (:`Update`
      (`SceneComponent.K2_SetWorldRotation` _cone (`KismetMathLibrary.RLerp` (`KismetMathLibrary.MakeRotator` _returnvalue_roll) (`KismetMathLibrary.MakeRotator` (* 45.0 _newtrack_0)) _newtrack_0) false false)
      (`KismetSystemLibrary.Delay` 0.2)
      (`self.Shoot`))
    (:`Finished`
      (goto _label :!via `PlayFromStart`))))

(fn `Shoot`
  (`|SpawnActorFromClass` "/Game/Blueprints/Projectiles/bpProjectileEnemy1.bpProjectileEnemy1_C" (`SceneComponent.K2_GetComponentToWorld` (`self.Scene`)) "Undefined" "OverrideRootScale" null 0.0 (0.0 -2000.0 0.0) (1.0 1.0 1.0)))

(fn `UserConstructionScript`
  (`parent.UserConstructionScript`))