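; Flamethrower enemy Blueprint that emits a flame particle effect following its ParticleSpawn point.
; BeginPlay runs the parent logic, waits briefly, then spawns P_Enemy_Flame at that point and stores the component.
; Tick teleports the emitter to ParticleSpawn's location, updating position only.
; Its valid-EnemyMesh branch wires straight back into that move, forming an unbroken loop within one tick; an invalid mesh prints a debug "Hello".
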(event `self.ReceiveBeginPlay`
  (`parent.ReceiveBeginPlay`)
  (`KismetSystemLibrary.Delay` 1.0)
  (bind _returnvalue (`GameplayStatics.SpawnEmitterAtLocation` "/Game/Blueprints/Projectiles/P_Enemy_Flame.P_Enemy_Flame" (`SceneComponent.K2_GetComponentLocation` (`self.ParticleSpawn`)))))

(event `self.ReceiveTick`
  (params (DeltaSeconds :type "Float (single-precision)"))
  (`SceneComponent.K2_SetWorldLocation` (stale `self.ReceiveBeginPlay` _returnvalue) (`SceneComponent.K2_GetComponentLocation` (`self.ParticleSpawn`)) true true :!label _label)
  (`/Engine/EditorBlueprintResources/StandardMacros.IsValid` (`self.EnemyMesh`)
    (:`Is Valid`
      (goto _label))
    (:`Is Not Valid`
      (`KismetSystemLibrary.PrintString` "Hello"))))

(fn `UserConstructionScript`
  (`parent.UserConstructionScript`))