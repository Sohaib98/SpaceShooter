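; BP_Enemy_SlingHighFrequency is an enemy that repeatedly fires high-frequency projectiles.
; Tick runs the parent logic, then a 0.5-second Delay, which ignores re-triggers while pending and so acts as a repeating timer for Shoot.
; Shoot spawns BP_ProjectileEnemy_HighFrequency at the Scene component's world transform, passing fixed damage, scale and a velocity along negative Y.
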(event `self.ReceiveBeginPlay`
  (`parent.ReceiveBeginPlay`))

(event `self.ReceiveTick`
  (params (DeltaSeconds :type "Float (single-precision)"))
  (`parent.ReceiveTick` DeltaSeconds)
  (`KismetSystemLibrary.Delay` 0.5)
  (`self.Shoot`))

(fn `Shoot`
  (`|SpawnActorFromClass` "/Game/Blueprints/Projectiles/BP_ProjectileEnemy_HighFrequency.BP_ProjectileEnemy_HighFrequency_C" (`SceneComponent.K2_GetComponentToWorld` (`self.Scene`)) "Undefined" "OverrideRootScale" null 10.0 (0.0 -2222.0 0.0) (2.0 2.0 2.0)))

(fn `UserConstructionScript`
  (`parent.UserConstructionScript`))