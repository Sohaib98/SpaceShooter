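; BP_Enemy_Drone is an enemy drone that eases its projectile-movement velocity toward zero while firing enemy projectiles.
; Tick plays a timeline whose updates lerp the velocity to a stop, then pass through a short Delay that paces calls to Shoot.
; Shoot spawns BpProjectileEnemy1 at the drone's transform with a fixed speed along negative Y and zero damage passed in.
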(event `self.ReceiveTick`
  (params (DeltaSeconds :type "Float (single-precision)"))
  (bind _projectilemovement (`self.ProjectileMovement`))
  (bind (_direction _newtrack_0) (`Timeline|Timeline_1_0`)
    (:`Update`
      (set `MovementComponent.Velocity` (`KismetMathLibrary.VLerp` (`MovementComponent.Velocity` _projectilemovement) (0.0 0.0 0.0) _newtrack_0) _projectilemovement)
      (`KismetSystemLibrary.Delay` 0.2)
      (`self.Shoot`))))

(fn `Shoot`
  (`|SpawnActorFromClass` "/Game/Blueprints/Projectiles/bpProjectileEnemy1.bpProjectileEnemy1_C" (`self.GetTransform`) "Undefined" "OverrideRootScale" null 0.0 (0.0 -2000.0 0.0) (1.0 1.0 1.0)))

(fn `UserConstructionScript`
  (`parent.UserConstructionScript`))