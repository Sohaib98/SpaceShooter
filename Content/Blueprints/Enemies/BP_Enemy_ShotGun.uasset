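; Shotgun-style enemy that repeatedly fires bursts of scattered projectiles along negative Y.
; Tick runs through a one-second Delay, which throttles the loop that calls Shoot several times per volley.
; Shoot spawns BpProjectileEnemy1 at the ProjectileSpawn component, randomizing Y/Z offset, roll, speed and scale to create the spread.
; Projectiles are spawned with zero Damage passed in.
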(event `self.ReceiveTick`
  (params (DeltaSeconds :type "Float (single-precision)"))
  (`KismetSystemLibrary.Delay` 1.0)
  (for _ (range 6)
    (`self.Shoot`)))

(fn `Shoot`
  (bind _returnvalue (`KismetMathLibrary.RandomFloatInRange` 0.5 2.0))
  (bind _returnvalue_2 (`SceneComponent.K2_GetComponentToWorld` (`self.ProjectileSpawn`)))
  (`|SpawnActorFromClass` "/Game/Blueprints/Projectiles/bpProjectileEnemy1.bpProjectileEnemy1_C" (`KismetMathLibrary.MakeTransform` (`KismetMathLibrary.MakeVector` (.x (.location _returnvalue_2)) (+ (.y (.location _returnvalue_2)) (`KismetMathLibrary.RandomFloatInRange` 0.0 200.0)) (+ (.z (.location _returnvalue_2)) (`KismetMathLibrary.RandomFloatInRange` 0.0 200.0))) (`KismetMathLibrary.MakeRotator` (`KismetMathLibrary.RandomFloatInRange` -10.0 10.0))) "Undefined" "OverrideRootScale" null 0.0 (`KismetMathLibrary.MakeVector` 0.0 (`KismetMathLibrary.RandomFloatInRange` -4000.0 -3000.0)) (`KismetMathLibrary.MakeVector` (`KismetMathLibrary.RandomFloatInRange` 0.5 2.0) (* _returnvalue 2.0) _returnvalue)))

(fn `UserConstructionScript`
  (`parent.UserConstructionScript`))