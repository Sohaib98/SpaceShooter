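; BP_Enemy_ISSCV is an enemy Blueprint carrying five child-actor turrets: an MK110, two torpedo launchers and two BulletStorms.
; On BeginPlay it runs the parent logic, then passes each turret component to a shared Turret function.
; That function casts the child actor to BP_Turret, clears its shoot flag and stops its timeline, so the turrets start with firing switched off.
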(event `self.ReceiveBeginPlay`
  (`parent.ReceiveBeginPlay`)
  (`|ExecutionSequence`
    (:`then_0`
      (`self.Turret` (`self.MK110`)))
    (:`then_1`
      (`self.Turret` (`self.TorpedoLauncher`)))
    (:`then_2`
      (`self.Turret` (`self.TorpedoLauncher2`)))
    (:`then_3`
      (`self.Turret` (`self.BulletStorm`)))
    (:`then_4`
      (`self.Turret` (`self.BulletStorm2`)))))

(fn `UserConstructionScript`
  (`parent.UserConstructionScript`))