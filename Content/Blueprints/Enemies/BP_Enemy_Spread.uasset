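; Enemy that fires a spread volley of BP_ProjectileEnemy shots along negative Y, roughly once per second.
; Tick calls the parent, then a Delay throttles the firing loop.
; Each shot spawns at ProjectileSpawn with an incrementing offset that staggers height and roll to form the fan.
; The first three shots get an overridden rotation rate, and every shot plays the EnemyShot sound at world origin.
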(event `self.ReceiveBeginPlay`
  (`parent.ReceiveBeginPlay`))

(event `self.ReceiveTick`
  (params (DeltaSeconds :type "Float (single-precision)"))
  (bind _returnvalue (* (`KismetMathLibrary.Conv_IntToDouble` (`self.Offset`)) 5.0))
  (`parent.ReceiveTick` DeltaSeconds)
  (`KismetSystemLibrary.Delay` 1.0)
  (set `self.Offset` (/ 5 -2))
  (for _index (range 6)
    (bind _returnvalue_2 (`|SpawnActorFromClass` "/Game/Blueprints/Projectiles/BP_ProjectileEnemy.BP_ProjectileEnemy_C" (`KismetMathLibrary.MakeTransform` (`KismetMathLibrary.MakeVector` (.x (.location (`SceneComponent.K2_GetComponentToWorld` (`self.ProjectileSpawn`)))) (.y (.location (`SceneComponent.K2_GetComponentToWorld` (`self.ProjectileSpawn`)))) (+ (.z (.location (`SceneComponent.K2_GetComponentToWorld` (`self.ProjectileSpawn`)))) _returnvalue)) (`KismetMathLibrary.MakeRotator` _returnvalue)) "AdjustIfPossibleButAlwaysSpawn" "OverrideRootScale" null 20.0 (0.0 -2200.0 0.0) (2.5 1.0 1.0)))
    (bind _output_get (set `/Game/Blueprints/Projectiles/BP_ProjectileEnemy.RotatingMovement` (`/Game/Blueprints/Projectiles/BP_ProjectileEnemy.RotatingMovement` _returnvalue_2) _returnvalue_2))
    (if (<= _index 2)
      (set `RotatingMovementComponent.RotationRate` (`KismetMathLibrary.MakeRotator` 0.0 -180.0) _output_get))
    (set `self.Offset` (+ (`self.Offset`) 1))
    (`GameplayStatics.PlaySoundAtLocation` "/Game/Audio/EnemyShot.EnemyShot")))

(fn `UserConstructionScript`
  (`parent.UserConstructionScript`))