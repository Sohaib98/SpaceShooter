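; Enemy actor that registers itself in the game mode's live count and travels along negative Y from its spawn point via a swept timeline lerp.
; Hitting the player deals damage and kills the enemy, sharing one death sequence with health depletion from incoming damage.
; Death decrements the count, adds score, rolls a random pickup drop, and plays explosion particles, sound and camera shake before destroying the actor.
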(event `self.ReceiveBeginPlay`
  (bind (_returnvalue_x _returnvalue_y _returnvalue_z) (`KismetMathLibrary.BreakVector` (`self.K2_GetActorLocation`)))
  (bind (_spawnlocation_x _spawnlocation_y) (`KismetMathLibrary.BreakVector` (`self.SpawnLocation`)))
  ;[1 1 1] Control  Random Move Direction
  (set `self.SpawnLocation` (`self.K2_GetActorLocation`))
  (bind _asbp_game_mode (cast `/Game/Blueprints/Misc/bpGameMode` (`GameplayStatics.GetGameMode`)))
  (bind _output_get (set `self.BpGameMode` _asbp_game_mode))
  (set `/Game/Blueprints/Misc/bpGameMode.LiveEnemies` (+ (`/Game/Blueprints/Misc/bpGameMode.LiveEnemies` _output_get) 1) _output_get)
  (bind (_direction _newtrack_0) (`Timeline|Timeline_0`)
    (:`Update`
      (`self.K2_SetActorLocation` (`KismetMathLibrary.VLerp` (`KismetMathLibrary.MakeVector` _returnvalue_x _returnvalue_y _returnvalue_z) (`KismetMathLibrary.MakeVector` _returnvalue_x (- _spawnlocation_y 6000.0) _returnvalue_z) _newtrack_0) true))))

(event `self.ReceiveHit`
  (params (MyComp :type "PrimitiveComponent Object Reference") (Other :type "Actor Object Reference") (OtherComp :type "PrimitiveComponent Object Reference") (bSelfMoved :type Boolean) (HitLocation :type "Vector Structure") (HitNormal :type "Vector Structure") (NormalImpulse :type "Vector Structure") (Hit :type "HitResult Structure (by ref)"))
  (bind _bpgamemode (`self.BpGameMode`))
  (bind _pickups (`self.PickUps`))
  ;[1 1 1] Death
  (cast `/Game/Blueprints/Enemies/BP_Enemy` Other
    (:`CastFailed`
      (set `self.bMoveDirection` (not (`self.bMoveDirection`)))
      (bind _asbp_player (cast `/Game/Blueprints/Misc/bpPlayer` Other))
      (`GameplayStatics.ApplyDamage` _asbp_player 25.0)
      (set `/Game/Blueprints/Misc/bpGameMode.LiveEnemies` (- (`/Game/Blueprints/Misc/bpGameMode.LiveEnemies` _bpgamemode) 1) _bpgamemode :!label _label)
      (`/Game/Blueprints/Misc/bpGameMode.AddScore` _bpgamemode)
      (if (<= (`KismetMathLibrary.RandomFloatInRange` 0.0 1.0) (`self.DropRate`))
        (`|SpawnActorFromClass` (`|GetArrayItem` _pickups (`KismetMathLibrary.RandomIntegerInRange` 0 (`KismetArrayLibrary.Array_LastIndex` _pickups))) (`self.GetTransform`) "Undefined" "OverrideRootScale"))
      (`GameplayStatics.SpawnEmitterAtLocation` "/Game/Art/Particles/pDeathEnemy.pDeathEnemy" (`self.K2_GetActorLocation`))
      (`/Game/Blueprints/Misc/bpGameMode.CallCamShake` (`self.BpGameMode`) "/Game/Blueprints/Misc/bpCamShakeExplosion.bpCamShakeExplosion_C")
      (`GameplayStatics.PlaySound2D` "/Game/Audio/Explosion.Explosion")
      (`self.K2_DestroyActor`))))

(event `self.ReceiveAnyDamage`
  (params (Damage :type "Float (single-precision)") (DamageType :type "DamageType Object Reference") (InstigatedBy :type "Controller Object Reference") (DamageCauser :type "Actor Object Reference"))
  ;[1 1 1] Death
  (set `self.Health` (`KismetMathLibrary.FClamp` (- (`self.Health`) Damage) 0.0 (`self.MaxHealth`)))
  (if (<= (`self.Health`) 0.0)
    (goto _label)))

(fn `Movement`
  (params (LocationY :type "Float (double-precision)") (LocationZ :type "Float (double-precision)") (Timeline :type "Float (double-precision)"))
  (bind _returnvalue_x (`KismetMathLibrary.BreakVector` (`self.K2_GetActorLocation`)))
  (`self.K2_SetActorLocation` (`KismetMathLibrary.VLerp` (`self.K2_GetActorLocation`) (`KismetMathLibrary.MakeVector` _returnvalue_x LocationY LocationZ) Timeline) true))

(fn `UserConstructionScript`
  (set `self.Health` (`self.MaxHealth`)))