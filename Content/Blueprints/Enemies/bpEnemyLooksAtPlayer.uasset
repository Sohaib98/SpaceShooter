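; Enemy actor that tilts toward the player once the player has entered its Box trigger.
; The overlap caches the bpPlayer reference, which is never cleared.
; Each Tick, after a zero-length Delay, it feeds the pitch of the look-at rotation to that player into the actor's roll, without checking the reference is valid.
; Projectile spawn and shot sound nodes are present but disconnected, so it never fires.
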(event `self.ReceiveBeginPlay`
  (`parent.ReceiveBeginPlay`))

(event `self.ReceiveTick`
  (params (DeltaSeconds :type "Float (single-precision)"))
  (`parent.ReceiveTick` DeltaSeconds)
  (`KismetSystemLibrary.Delay` 0.0)
  (bind (_returnvalue_roll _returnvalue_pitch) (`KismetMathLibrary.BreakRotator` (`KismetMathLibrary.FindLookAtRotation` (`self.K2_GetActorLocation`) (`self.K2_GetActorLocation` (stale `self.Box.OnComponentBeginOverlap` _asbp_player)))))
  (`self.K2_SetActorRotation` (`KismetMathLibrary.MakeRotator` (+ _returnvalue_pitch 0.0))))

(event `self.Box.OnComponentBeginOverlap`
  (params (OverlappedComponent :type "PrimitiveComponent Object Reference") (OtherActor :type "Actor Object Reference") (OtherComp :type "PrimitiveComponent Object Reference") (OtherBodyIndex :type Integer) (bFromSweep :type Boolean) (SweepResult :type "HitResult Structure (by ref)"))
  (bind _asbp_player (cast `/Game/Blueprints/Misc/bpPlayer` OtherActor)))

(fn `UserConstructionScript`
  (`parent.UserConstructionScript`))