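; Hunter drone enemy Blueprint that continuously fires twin machine guns.
; Tick runs through a 0.2-second Delay as a fire-rate gate before calling ShootMG.
; ShootMG spawns zero-damage, half-scale BP_ProjectileEnemy actors at the left and right spawn components with a fixed speed vector.
; A shot counter wraps at ten but drives no other behavior here.
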(event `self.ReceiveBeginPlay`)

(event `self.ReceiveTick`
  (params (DeltaSeconds :type "Float (single-precision)"))
  (`KismetSystemLibrary.Delay` 0.2)
  (`self.ShootMG`))

(fn `ShootMG`
  (`|SpawnActorFromClass` "/Game/Blueprints/Projectiles/BP_ProjectileEnemy.BP_ProjectileEnemy_C" (`SceneComponent.K2_GetComponentToWorld` (`self.MJGProjectileSpawnLeft`)) "Undefined" "OverrideRootScale" null 0.0 (0.0 2000.0 0.0) (0.5 0.5 0.5))
  (`|SpawnActorFromClass` "/Game/Blueprints/Projectiles/BP_ProjectileEnemy.BP_ProjectileEnemy_C" (`SceneComponent.K2_GetComponentToWorld` (`self.MJGProjectileSpawRight`)) "Undefined" "OverrideRootScale" null 0.0 (0.0 2000.0 0.0) (0.5 0.5 0.5))
  (set `self.IMGShots` (+ (`self.IMGShots`) 1))
  (if (>= (`self.IMGShots`) 10)
    (set `self.IMGShots` 0)))

(fn `UserConstructionScript`)