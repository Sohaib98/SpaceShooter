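; Hunter drone enemy that continuously alternates between rocket volleys and twin machine-gun bursts, without any targeting logic.
; Tick branches on a rocket-mode flag, using Delay nodes to throttle each weapon's fire rate.
; Rockets launch in sequence from six stored mount points, while the gun fires paired shots from left and right spawns.
; Both weapons spawn the same enemy projectile with different speed and scale, flipping modes via shot counters.
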(event `self.ReceiveBeginPlay`
  (set `self.RocketArray` (`|MakeArray` (`self.Rocket1`) (`self.Rocket2`) (`self.Rocket3`) (`self.Rocket4`) (`self.Rocket5`) (`self.Rocket6`))))

(event `self.ReceiveTick`
  (params (DeltaSeconds :type "Float (single-precision)"))
  (if (`self.BRockets`)
    (`KismetSystemLibrary.Delay` 0.4)
    (`self.ShootRockets`)
    (else
      (`KismetSystemLibrary.Delay` 0.2)
      (`self.ShootMG`))))

(fn `ShootMG`
  (`|SpawnActorFromClass` "/Game/Blueprints/Projectiles/BP_ProjectileEnemy.BP_ProjectileEnemy_C" (`SceneComponent.K2_GetComponentToWorld` (`self.MJGProjectileSpawnLeft`)) "Undefined" "OverrideRootScale" null 0.0 (0.0 2000.0 0.0) (0.5 0.5 0.5))
  (`|SpawnActorFromClass` "/Game/Blueprints/Projectiles/BP_ProjectileEnemy.BP_ProjectileEnemy_C" (`SceneComponent.K2_GetComponentToWorld` (`self.MJGProjectileSpawRight`)) "Undefined" "OverrideRootScale" null 0.0 (0.0 2000.0 0.0) (0.5 0.5 0.5))
  (set `self.IMGShots` (+ (`self.IMGShots`) 1))
  (if (>= (`self.IMGShots`) 10)
    (set `self.IMGShots` 0)
    (set `self.BRockets` true)))

(fn `ShootRockets`
  (`|SpawnActorFromClass` "/Game/Blueprints/Projectiles/BP_ProjectileEnemy.BP_ProjectileEnemy_C" (`SceneComponent.K2_GetComponentToWorld` (`|GetArrayItem` (`self.RocketArray`) (`self.IRocketIndex`))) "Undefined" "OverrideRootScale" null 0.0 (0.0 1000.0 0.0) (1.0 2.0 1.0))
  (set `self.IRocketIndex` (+ (`self.IRocketIndex`) 1))
  (if (>= (`self.IRocketIndex`) 6)
    (set `self.IRocketIndex` 0)
    (set `self.BRockets` false)))

(fn `UserConstructionScript`)