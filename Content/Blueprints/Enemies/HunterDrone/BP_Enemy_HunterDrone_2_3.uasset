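; Hunter drone enemy that sweeps along world Y and fires twin machine-gun projectiles.
; After a start delay, it caches its spawn transform and repeatedly replays a timeline that lerps Y from that origin, pausing between runs.
; Tick uses Delay nodes to clear the moving flag, then throttle ShootMG, which spawns projectiles at left and right muzzles and wraps a shot counter.
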(event `self.ReceiveBeginPlay`
  (bind _tbegintransform (`self.TBeginTransform`))
  (`KismetSystemLibrary.Delay` 2.0)
  (set `self.TBeginTransform` (`self.GetTransform`))
  (`KismetSystemLibrary.Delay` 5.0 :!label _label)
  (bind (_direction _newtrack_1) (`Timeline|Timeline_1` :!via `PlayFromStart`)
    (:`Update`
      (`self.K2_SetActorLocation` (`KismetMathLibrary.VLerp` (`KismetMathLibrary.MakeVector` (.x (.location _tbegintransform)) (.y (.location _tbegintransform)) (.z (.location _tbegintransform))) (`KismetMathLibrary.MakeVector` (.x (.location _tbegintransform)) (* _newtrack_1 (+ (.y (.location _tbegintransform)) 8000.0)) (.z (.location _tbegintransform))) _newtrack_1) true))
    (:`Finished`
      (goto _label))))

(event `self.ReceiveTick`
  (params (DeltaSeconds :type "Float (single-precision)"))
  (if (`self.BMoving`)
    (`KismetSystemLibrary.Delay` 8.0)
    (set `self.BMoving` false)
    (else
      (`KismetSystemLibrary.Delay` 0.2)
      (`self.ShootMG`))))

(fn `ShootMG`
  (`|SpawnActorFromClass` "/Game/Blueprints/Projectiles/BP_ProjectileEnemy.BP_ProjectileEnemy_C" (`SceneComponent.K2_GetComponentToWorld` (`self.MJGProjectileSpawnLeft`)) "Undefined" "OverrideRootScale" null 0.0 (0.0 4000.0 0.0) (0.5 0.5 0.5))
  (`|SpawnActorFromClass` "/Game/Blueprints/Projectiles/BP_ProjectileEnemy.BP_ProjectileEnemy_C" (`SceneComponent.K2_GetComponentToWorld` (`self.MJGProjectileSpawRight`)) "Undefined" "OverrideRootScale" null 0.0 (0.0 4000.0 0.0) (0.5 0.5 0.5))
  (set `self.IMGShots` (+ (`self.IMGShots`) 1))
  (if (>= (`self.IMGShots`) 10)
    (set `self.IMGShots` 0)))

(fn `UserConstructionScript`)