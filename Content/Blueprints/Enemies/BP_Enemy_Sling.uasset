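; Sling enemy that swings its Cone and continuously fires enemy projectiles from its Scene component's transform.
; A Timeline started on BeginPlay drives the Cone's roll up to a 45-degree scale, replaying in reverse from the end whenever it finishes.
; Tick feeds a Delay that throttles Shoot to about four BP_ProjectileEnemy spawns per second, with fixed damage and velocity.
; RotateCounterClockWise is defined but never called here.
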(event `self.ReceiveBeginPlay`
  (`parent.ReceiveBeginPlay`)
  (bind (_direction _newtrack_0) (`Timeline|Timeline_0_0` :!via `PlayFromStart` :!label _label)
    (:`Update`
      (`self.RotateClockWise` _newtrack_0))
    (:`Finished`
      (goto _label :!via `ReverseFromEnd`))))

(event `self.ReceiveTick`
  (params (DeltaSeconds :type "Float (single-precision)"))
  (`parent.ReceiveTick` DeltaSeconds)
  (`KismetSystemLibrary.Delay` 0.25)
  (`self.Shoot`))

(fn `RotateClockWise`
  (params (TimeLine :type "Float (double-precision)"))
  (bind _cone (`self.Cone`))
  (bind _returnvalue_roll (`KismetMathLibrary.BreakRotator` (`SceneComponent.K2_GetComponentRotation` _cone)))
  (`SceneComponent.K2_SetRelativeRotation` _cone (`KismetMathLibrary.MakeRotator` (`KismetMathLibrary.Lerp` _returnvalue_roll (* TimeLine 45.0) 1.0) 0.0) false false))

(fn `RotateCounterClockWise`
  (params (TimeLine :type "Float (double-precision)"))
  (bind _cone (`self.Cone`))
  (bind _returnvalue_roll (`KismetMathLibrary.BreakRotator` (`SceneComponent.K2_GetComponentRotation` _cone)))
  (`SceneComponent.K2_SetRelativeRotation` _cone (`KismetMathLibrary.MakeRotator` (`KismetMathLibrary.Lerp` _returnvalue_roll -45.0 TimeLine) 0.0) false false))

(fn `Shoot`
  (`|SpawnActorFromClass` "/Game/Blueprints/Projectiles/BP_ProjectileEnemy.BP_ProjectileEnemy_C" (`SceneComponent.K2_GetComponentToWorld` (`self.Scene`)) "Undefined" "OverrideRootScale" null 10.0 (0.0 -2222.0 0.0) (2.0 2.0 2.0)))

(fn `UserConstructionScript`
  (`parent.UserConstructionScript`))