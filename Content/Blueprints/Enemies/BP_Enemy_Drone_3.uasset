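; Enemy drone that brakes to a stop and fires radial bursts of projectiles.
; Tick plays a timeline that lerps ProjectileMovement velocity toward zero, and each update feeds a one-second Delay that gates the shot loop.
; Each Shoot call spawns a BpProjectileEnemy1 at the drone, stepping roll by shot index times 360 / IMaxShots to fan the shots around a circle.
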(event `self.ReceiveTick`
  (params (DeltaSeconds :type "Float (single-precision)"))
  (bind _projectilemovement (`self.ProjectileMovement`))
  (bind (_direction _newtrack_0) (`Timeline|Timeline_1`)
    (:`Update`
      (set `MovementComponent.Velocity` (`KismetMathLibrary.VLerp` (`MovementComponent.Velocity` _projectilemovement) (0.0 0.0 0.0) _newtrack_0) _projectilemovement)
      (`KismetSystemLibrary.Delay` 1.0)
      (for _index (range (+ (`self.IMaxShots`) 1))
        (`self.Shoot` _index)))))

(fn `Shoot`
  (params (IShotCount :type Integer))
  (bind _returnvalue (`self.GetTransform`))
  (`|SpawnActorFromClass` "/Game/Blueprints/Projectiles/bpProjectileEnemy1.bpProjectileEnemy1_C" (`KismetMathLibrary.MakeTransform` (.location _returnvalue) (`KismetMathLibrary.MakeRotator` (* IShotCount (`KismetMathLibrary.Conv_IntToDouble` (/ 360 (`self.IMaxShots`)))) (.pitch (.rotation _returnvalue)) (.yaw (.rotation _returnvalue))) (.scale _returnvalue)) "Undefined" "OverrideRootScale" null 0.0 (0.0 -2000.0 0.0) (1.0 1.0 1.0))
  (set `self.FRotation` 0.0))

(fn `UserConstructionScript`
  (`parent.UserConstructionScript`))