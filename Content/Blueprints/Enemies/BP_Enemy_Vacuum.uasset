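; Vacuum enemy that sucks the player toward its mesh when the player enters its Cone volume.
; The cone's begin overlap casts to bpPlayer and plays a timeline that moves the player with sweep on each update.
; Each step lerps from the player's current location toward the mesh's Y and Z by the timeline alpha, leaving X untouched.
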(event `self.Cone.OnComponentBeginOverlap`
  (params (OverlappedComponent :type "PrimitiveComponent Object Reference") (OtherActor :type "Actor Object Reference") (OtherComp :type "PrimitiveComponent Object Reference") (OtherBodyIndex :type Integer) (bFromSweep :type Boolean) (SweepResult :type "HitResult Structure (by ref)"))
  (bind (_returnvalue_x _returnvalue_y _returnvalue_z) (`KismetMathLibrary.BreakVector` (`SceneComponent.K2_GetComponentLocation` (`self.EnemyMesh`))))
  (bind _asbp_player (cast `/Game/Blueprints/Misc/bpPlayer` OtherActor))
  (bind (_direction _newtrack_0) (`Timeline|Timeline_1`)
    (:`Update`
      (bind (_returnvalue_x_2 _returnvalue_y_2 _returnvalue_z_2) (`KismetMathLibrary.BreakVector` (`self.K2_GetActorLocation` _asbp_player)))
      (`self.K2_SetActorLocation` _asbp_player (`KismetMathLibrary.VLerp` (`KismetMathLibrary.MakeVector` _returnvalue_x_2 _returnvalue_y_2 _returnvalue_z_2) (`KismetMathLibrary.MakeVector` _returnvalue_x_2 _returnvalue_y _returnvalue_z) _newtrack_0) true false))))

(fn `UserConstructionScript`
  (`parent.UserConstructionScript`))