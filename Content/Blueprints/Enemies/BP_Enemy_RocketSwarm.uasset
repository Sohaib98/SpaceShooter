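; Rocket swarm enemy that fires repeating volleys of five BP_ProjectileEnemy projectiles along negative Y.
; Tick uses Delay nodes as a cadence timer, spacing shots briefly apart and pausing longer before resetting the shot counter.
; Shoot spawns each projectile from the ProjectileSpawn transform, stepping progressively lower in Z with the counter to form a vertical column.
; Projectiles spawn with elongated scale and zero Damage.
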(event `self.ReceiveTick`
  (params (DeltaSeconds :type "Float (single-precision)"))
  (bind _ishot (`self.IShot`))
  (if (>= (`self.IShot`) 5)
    (`KismetSystemLibrary.Delay` 5.0)
    (set `self.IShot` 0)
    (else
      (`KismetSystemLibrary.Delay` 0.25)
      (`self.Shoot` (* _ishot -200.0))
      (set `self.IShot` (+ _ishot 1)))))

(fn `Shoot`
  (params (FHeight :type "Float (double-precision)"))
  (bind _returnvalue (`SceneComponent.K2_GetComponentToWorld` (`self.ProjectileSpawn`)))
  (`|SpawnActorFromClass` "/Game/Blueprints/Projectiles/BP_ProjectileEnemy.BP_ProjectileEnemy_C" (`KismetMathLibrary.MakeTransform` (`KismetMathLibrary.MakeVector` (.x (.location _returnvalue)) (.y (.location _returnvalue)) (+ (.z (.location _returnvalue)) FHeight)) (.rotation _returnvalue) (.scale _returnvalue)) "Undefined" "OverrideRootScale" null 0.0 (0.0 -2000.0 0.0) (2.0 4.0 2.0)))

(fn `UserConstructionScript`
  (`parent.UserConstructionScript`))