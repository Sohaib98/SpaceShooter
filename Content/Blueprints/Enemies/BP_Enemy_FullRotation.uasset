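; Enemy actor that continuously spins its cone while firing a stream of enemy projectiles.
; Each Tick runs the parent logic, then sets the Cone's relative roll to its world roll plus a fixed step, so spin rate depends on frame rate.
; Shoot then spawns a BP_ProjectileEnemy at the Scene component's world transform every frame, with fixed speed and zero damage.
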(event `self.ReceiveTick`
  (params (DeltaSeconds :type "Float (single-precision)"))
  (bind _cone (`self.Cone`))
  (bind _returnvalue_roll (`KismetMathLibrary.BreakRotator` (`SceneComponent.K2_GetComponentRotation` _cone)))
  (`parent.ReceiveTick` DeltaSeconds)
  (`SceneComponent.K2_SetRelativeRotation` _cone (`KismetMathLibrary.MakeRotator` (+ _returnvalue_roll 1.0) 0.0) false false)
  (`self.Shoot`))

(fn `Shoot`
  (`|SpawnActorFromClass` "/Game/Blueprints/Projectiles/BP_ProjectileEnemy.BP_ProjectileEnemy_C" (`SceneComponent.K2_GetComponentToWorld` (`self.Scene`)) "Undefined" "OverrideRootScale" null 0.0 (0.0 2222.0 0.0) (1.0 1.0 1.0)))

(fn `UserConstructionScript`
  (`parent.UserConstructionScript`))