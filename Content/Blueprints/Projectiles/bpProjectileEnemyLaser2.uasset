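; Enemy laser projectile that stretches as it travels along negative world Y and damages the player on contact.
; Each Tick moves it by a step proportional to its Y scale, while a timeline lengthens that scale, so speed follows the stretch.
; Any mesh overlap destroys it; player hits also call ApplyDamage without the unused Damage variable, spawn a hit emitter and trigger camera shake through bpGameMode.
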(event `self.ReceiveTick`
  (params (DeltaSeconds :type "Float (single-precision)"))
  (bind (_returnvalue_x _returnvalue_y _returnvalue_z) (`KismetMathLibrary.BreakVector` (`self.K2_GetActorLocation`)))
  (bind (_returnvalue_x_2 _returnvalue_y_2) (`KismetMathLibrary.BreakVector` (`self.GetActorScale3D`)))
  ;[1 1 1] Move Projectile
  (`self.K2_SetActorLocation` (`KismetMathLibrary.MakeVector` _returnvalue_x (- _returnvalue_y (* _returnvalue_y_2 10.0)) _returnvalue_z))
  (bind (_direction _newtrack_0) (`Timeline|Timeline_0`)
    (:`Update`
      (`self.SetActorRelativeScale3D` (`KismetMathLibrary.VLerp` (1.0 1.0 1.0) (1.0 200.0 1.0) _newtrack_0)))))

(event `self.StaticMesh.OnComponentBeginOverlap`
  (params (OverlappedComponent :type "PrimitiveComponent Object Reference") (OtherActor :type "Actor Object Reference") (OtherComp :type "PrimitiveComponent Object Reference") (OtherBodyIndex :type Integer) (bFromSweep :type Boolean) (SweepResult :type "HitResult Structure (by ref)"))
  ;[1 1 1] Collision Events
  (bind _asbp_player (cast `/Game/Blueprints/Misc/bpPlayer` OtherActor)
    (:`then`
      (`GameplayStatics.ApplyDamage` _asbp_player)
      (`GameplayStatics.SpawnEmitterAtLocation` "/Game/Art/Particles/pHitPlayer.pHitPlayer" (`self.K2_GetActorLocation`))
      (bind _asbp_game_mode (cast `/Game/Blueprints/Misc/bpGameMode` (`GameplayStatics.GetGameMode`)))
      (`/Game/Blueprints/Misc/bpGameMode.CallCamShake` _asbp_game_mode "/Game/Blueprints/Misc/bpCamShakeCollision.bpCamShakeCollision_C"))
    (:`CastFailed`
      _))
  (`self.K2_DestroyActor`))

(fn `UserConstructionScript`)