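; BP_EnemyProjectile_Sword is an enemy projectile actor that forms a lengthening blade, with no collision response or damage logic in its graph.
; Each Tick adds a fixed step to the Cube's Y scale, so growth is unbounded and frame-rate dependent.
; The Cube's bounds extent offsets it along negative world Y, and twice that places the Sphere at the tip.
; Both positions are absolute world coordinates, independent of the actor's location.
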(event `self.ReceiveTick`
  (params (DeltaSeconds :type "Float (single-precision)"))
  (bind _cube (`self.Cube`))
  (bind _cube_2 (`self.Cube`))
  (bind (_returnvalue_x _returnvalue_y) (`KismetMathLibrary.BreakVector` (`SceneComponent.K2_GetComponentScale` _cube_2)))
  (bind _returnvalue (- 0.0 (.y (`.BoxExtent` (`KismetSystemLibrary.GetComponentBounds` _cube)))))
  (`SceneComponent.K2_SetWorldLocation` _cube (`KismetMathLibrary.MakeVector` 0.0 _returnvalue) false false)
  (`SceneComponent.SetWorldScale3D` _cube_2 (`KismetMathLibrary.MakeVector` 1.0 (+ _returnvalue_y 0.05) 1.0))
  (`SceneComponent.K2_SetWorldLocation` (`self.Sphere`) (`KismetMathLibrary.MakeVector` 0.0 (* _returnvalue 2.0)) false false))

(fn `UserConstructionScript`)