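; Enemy rocket projectile that homes on the player and destroys itself when its cone overlaps them.
; The start box stores the first overlapping player, and the end box clears FollowPlayer when the player enters it.
; While following, Tick blends movement velocity toward the normalized player-to-rocket offset scaled by IncreasedSpeed, so the sign of that speed sets the direction.
; Look-at rotation and move-to nodes are unconnected.
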(event `self.ReceiveTick`
  (params (DeltaSeconds :type "Float (single-precision)"))
  ;[1 1 1] Move towards player
  (`/Engine/EditorBlueprintResources/StandardMacros.IsValid` (`self.Player`)
    (:`Is Valid`
      (if (`self.FollowPlayer`)
        (set `MovementComponent.Velocity` (`KismetMathLibrary.VLerp` (`MovementComponent.Velocity` (`self.ProjectileMovement`)) (* (`KismetMathLibrary.Normal` (- (`self.K2_GetActorLocation`) (`self.K2_GetActorLocation` (`self.Player`)))) (`self.IncreasedSpeed`)) 0.125) (`self.ProjectileMovement`))))))

(event `self.HomibngEndBox.OnComponentBeginOverlap`
  (params (OverlappedComponent :type "PrimitiveComponent Object Reference") (OtherActor :type "Actor Object Reference") (OtherComp :type "PrimitiveComponent Object Reference") (OtherBodyIndex :type Integer) (bFromSweep :type Boolean) (SweepResult :type "HitResult Structure (by ref)"))
  ;[1 1 1] Move towards player
  (cast `/Game/Blueprints/Misc/bpPlayer` OtherActor)
  (set `self.FollowPlayer` false))

(event `self.HomingStartBox.OnComponentBeginOverlap`
  (params (OverlappedComponent :type "PrimitiveComponent Object Reference") (OtherActor :type "Actor Object Reference") (OtherComp :type "PrimitiveComponent Object Reference") (OtherBodyIndex :type Integer) (bFromSweep :type Boolean) (SweepResult :type "HitResult Structure (by ref)"))
  ;[1 1 1] Rotate towards player
  (bind _asbp_player (cast `/Game/Blueprints/Misc/bpPlayer` OtherActor))
  (`/Engine/EditorBlueprintResources/StandardMacros.IsValid` (`self.Player`)
    (:`Is Not Valid`
      (bind _output_get (set `self.Player` _asbp_player)))))

(event `self.Cone.OnComponentBeginOverlap`
  (params (OverlappedComponent :type "PrimitiveComponent Object Reference") (OtherActor :type "Actor Object Reference") (OtherComp :type "PrimitiveComponent Object Reference") (OtherBodyIndex :type Integer) (bFromSweep :type Boolean) (SweepResult :type "HitResult Structure (by ref)"))
  ;[1 1 1] Hit Player
  (cast `/Game/Blueprints/Misc/bpPlayer` OtherActor)
  (`self.K2_DestroyActor`))

(fn `UserConstructionScript`)