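; Enemy laser projectile: a beam that stretches along Y and hits the player on overlap.
; Each tick it grows its Y scale and recenters from its bounds, keeping one end fixed so it extends toward negative Y.
; Player overlaps call ApplyDamage with no amount set, spawn a hit emitter and request camera shake; any overlap destroys it, unless the game mode cast fails.
; Construction applies a glowing dynamic enemy material.
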(event `self.ReceiveTick`
  (params (DeltaSeconds :type "Float (single-precision)"))
  (bind (_returnvalue_x _returnvalue_y _returnvalue_z) (`KismetMathLibrary.BreakVector` (`self.K2_GetActorLocation`)))
  (bind (_returnvalue_x_2 _returnvalue_y_2) (`KismetMathLibrary.BreakVector` (`self.GetActorScale3D`)))
  ;[1 1 1] Move Projectile
  (`self.SetActorScale3D` (`KismetMathLibrary.MakeVector` 1.0 (+ _returnvalue_y_2 1.0) 1.0))
  (`self.K2_SetActorLocation` (`KismetMathLibrary.MakeVector` _returnvalue_x (* (- (.y (`.BoxExtent` (`self.GetActorBounds` false))) 2500.0) -1.0) _returnvalue_z)))

(event `self.StaticMesh.OnComponentBeginOverlap`
  (params (OverlappedComponent :type "PrimitiveComponent Object Reference") (OtherActor :type "Actor Object Reference") (OtherComp :type "PrimitiveComponent Object Reference") (OtherBodyIndex :type Integer) (bFromSweep :type Boolean) (SweepResult :type "HitResult Structure (by ref)"))
  ;[1 1 1] Collision Events
  (bind _asbp_player (cast `/Game/Blueprints/Misc/bpPlayer` OtherActor)
    (:`then`
      (`GameplayStatics.ApplyDamage` _asbp_player)
      (`GameplayStatics.SpawnEmitterAtLocation` "/Game/Art/Particles/pHitPlayer.pHitPlayer" (`self.K2_GetActorLocation`))
      (bind _asbp_game_mode (cast `/Game/Blueprints/Misc/bpGameMode` (`GameplayStatics.GetGameMode`)))
      (`/Game/Blueprints/Misc/bpGameMode.CallCamShake` _asbp_game_mode "/Game/Blueprints/Misc/bpCamShakeCollision.bpCamShakeCollision_C"))
    (:`CastFailed`
      _))
  (`self.K2_DestroyActor`))

(fn `UserConstructionScript`
  (bind _returnvalue (`PrimitiveComponent.CreateDynamicMaterialInstance` (`self.StaticMesh`) 0 "/Game/Art/Materials/mEnemy.mEnemy"))
  (`MaterialInstanceDynamic.SetScalarParameterValue` _returnvalue "Light" 50.0))