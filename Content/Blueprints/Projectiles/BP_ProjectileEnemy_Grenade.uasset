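; Enemy grenade projectile that spins along the world Y axis, then bursts into a particle effect and disappears without applying damage in this graph.
; A timeline started on BeginPlay eases speed and spin rate toward fixed end values.
; Tick applies both per frame without delta-time scaling, using a swept move.
; A five-second Delay within Tick acts as the fuse before spawning the emitter and destroying the actor.
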(event `self.ReceiveBeginPlay`
  (bind (_direction _newtrack_0) (`Timeline|Timeline_0`)
    (:`Update`
      (set `self.FSpeed` (`KismetMathLibrary.Lerp` (`self.FSpeed`) -1.0 _newtrack_0))
      (set `self.FRotationRate` (`KismetMathLibrary.Lerp` (`self.FRotationRate`) 0.5 _newtrack_0)))))

(event `self.ReceiveTick`
  (params (DeltaSeconds :type "Float (single-precision)"))
  (bind (_returnvalue_roll _returnvalue_pitch _returnvalue_yaw) (`KismetMathLibrary.BreakRotator` (`self.K2_GetActorRotation`)))
  (bind (_returnvalue_x _returnvalue_y _returnvalue_z) (`KismetMathLibrary.BreakVector` (`self.K2_GetActorLocation`)))
  (`self.K2_SetActorLocation` (`KismetMathLibrary.MakeVector` _returnvalue_x (+ _returnvalue_y (`self.FSpeed`)) _returnvalue_z) true)
  (`self.K2_SetActorRotation` (`KismetMathLibrary.MakeRotator` (+ _returnvalue_roll (`self.FRotationRate`)) 0.0 (+ _returnvalue_yaw (`self.FRotationRate`))))
  (`KismetSystemLibrary.Delay` 5.0)
  (`GameplayStatics.SpawnEmitterAtLocation` "/Game/Art/Particles/pHitEnemy.pHitEnemy" (`self.K2_GetActorLocation`))
  (`self.K2_DestroyActor`))

(fn `UserConstructionScript`
  (`parent.UserConstructionScript`))