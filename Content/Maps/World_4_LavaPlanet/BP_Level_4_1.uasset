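; BP_Level_4_1 is an actor for Level 4_1 of the Lava Planet world that manages that level's planet and sky sphere.
; BeginPlay spawns BP_LavaPlanet and a cloudless sky sphere at fixed world transforms.
; Tick copies this actor's scale onto both every frame, overriding their spawn scales, including the sky sphere's enlarged one.
; Destroying the actor also destroys both spawned actors.
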(event `self.ReceiveTick`
  (params (DeltaSeconds :type "Float (single-precision)"))
  (bind _returnvalue (`self.GetActorScale3D`))
  (`self.SetActorScale3D` (stale `self.ReceiveBeginPlay` _returnvalue) _returnvalue)
  (`self.SetActorScale3D` (stale `self.ReceiveBeginPlay` _returnvalue_2) _returnvalue))

(event `self.ReceiveBeginPlay`
  (bind _returnvalue (`|SpawnActorFromClass` "/Game/Maps/World_4_LavaPlanet/BP_LavaPlanet.BP_LavaPlanet_C" (`KismetMathLibrary.MakeTransform` (17100.0 130.0 -10000.0) (struct) (1.0 1.0 1.0)) "Undefined" "OverrideRootScale"))
  (bind _returnvalue_2 (`|SpawnActorFromClass` "/Game/Maps/World_4_LavaPlanet/BP_Sky_Sphere_NoClouds_Level_4_1.BP_Sky_Sphere_NoClouds_Level_4_1_C" (`KismetMathLibrary.MakeTransform` (0.0 0.0 0.0) (struct) (1000.0 1000.0 1000.0)) "Undefined" "OverrideRootScale")))

(event `self.ReceiveDestroyed`
  (`self.K2_DestroyActor` (stale `self.ReceiveBeginPlay` _returnvalue))
  (`self.K2_DestroyActor` (stale `self.ReceiveBeginPlay` _returnvalue_2)))

(fn `UserConstructionScript`)