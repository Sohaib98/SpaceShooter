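; BP_Level_4_2 is a level actor for the World 4 lava planet that manages the volcano and sky sphere scenery.
; On BeginPlay it spawns both actors at fixed world transforms and keeps references to them.
; Every Tick copies its own scale onto both without moving them, and its Destroyed event destroys them along with it.
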(event `self.ReceiveTick`
  (params (DeltaSeconds :type "Float (single-precision)"))
  (bind _returnvalue (`self.GetActorScale3D`))
  (`self.SetActorScale3D` (stale `self.ReceiveBeginPlay` _returnvalue) _returnvalue)
  (`self.SetActorScale3D` (stale `self.ReceiveBeginPlay` _returnvalue_2) _returnvalue))

(event `self.ReceiveBeginPlay`
  (bind _returnvalue (`|SpawnActorFromClass` "/Game/Maps/World_4_LavaPlanet/BP_VolcanoSolo.BP_VolcanoSolo_C" (`KismetMathLibrary.MakeTransform` (21560.0 -1020.0 -4370.0) (struct) (1.0 1.0 1.0)) "Undefined" "OverrideRootScale"))
  (bind _returnvalue_2 (`|SpawnActorFromClass` "/Game/Maps/World_4_LavaPlanet/BP_Sky_Sphere_Level_4_1.BP_Sky_Sphere_Level_4_1_C" (`KismetMathLibrary.MakeTransform` (0.0 0.0 0.0)) "Undefined" "OverrideRootScale")))

(event `self.ReceiveDestroyed`
  (`self.K2_DestroyActor` (stale `self.ReceiveBeginPlay` _returnvalue))
  (`self.K2_DestroyActor` (stale `self.ReceiveBeginPlay` _returnvalue_2)))

(fn `UserConstructionScript`)