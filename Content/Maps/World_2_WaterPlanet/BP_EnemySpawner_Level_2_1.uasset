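; Enemy spawner for level 2-1 of the Water Planet world, spawning scripted enemy waves, including a mid-sequence boss.
; WaveCheck switches on WaveIndex when CheckWave passes, runs that wave's collapsed spawn graph, then calls IncrementWave.
; Some waves stagger spawns with delays, offset enemies vertically with replaying timelines, or spawn follow-ups from OnDestroyed before advancing.
; Several wave graphs and the AllEnemiesDefeated call are unwired.
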(event `OnDestroyed_Event_1` :!signature `self.OnDestroyed`
  (params (DestroyedActor :type "Actor Object Reference"))
  (`|SpawnActorFromClass` "/Game/Blueprints/Enemies/BP_Enemy_FlameThrower.BP_Enemy_FlameThrower_C" (`KismetMathLibrary.MakeTransform` (- (`self.VTop`) (0.0 0.0 500.0)) (struct) (1.0 -1.0 1.0)) "Undefined" "OverrideRootScale")
  (`|SpawnActorFromClass` "/Game/Blueprints/Enemies/BP_Enemy_FlameThrower.BP_Enemy_FlameThrower_C" (`KismetMathLibrary.MakeTransform` (+ (`self.VBottom`) (0.0 0.0 500.0)) (struct) (1.0 -1.0 1.0)) "Undefined" "OverrideRootScale")
  (`self.IncrementWave` :!label _label))

(event `OnDestroyed_Event_2` :!signature `self.OnDestroyed`
  (params (DestroyedActor :type "Actor Object Reference"))
  (`|SpawnActorFromClass` "/Game/Blueprints/Enemies/BP_Enemy_FullRotationNoise.BP_Enemy_FullRotationNoise_C" (`KismetMathLibrary.MakeTransform` (`self.VTop`) (struct) (1.0 -1.0 1.0)) "Undefined" "OverrideRootScale")
  (`|SpawnActorFromClass` "/Game/Blueprints/Enemies/BP_Enemy_FullRotationNoise.BP_Enemy_FullRotationNoise_C" (`KismetMathLibrary.MakeTransform` (`self.VBottom`) (struct) (1.0 -1.0 1.0)) "Undefined" "OverrideRootScale")
  (`|SpawnActorFromClass` "/Game/Blueprints/Enemies/BP_Enemy_FullRotation.BP_Enemy_FullRotation_C" (`KismetMathLibrary.MakeTransform` (`self.VCenter`) (struct) (1.0 -1.0 1.0)) "Undefined" "OverrideRootScale"))

(event `OnDestroyed_Event_0` :!signature `self.OnDestroyed`
  (params (DestroyedActor :type "Actor Object Reference"))
  (`|SpawnActorFromClass` "/Game/Blueprints/Enemies/BP_Enemy_FullBounce.BP_Enemy_FullBounce_C" (`KismetMathLibrary.MakeTransform` (`self.VTop`) (struct) (1.0 -1.0 1.0)) "Undefined" "OverrideRootScale")
  (`|SpawnActorFromClass` "/Game/Blueprints/Enemies/BP_Enemy_FullBounce.BP_Enemy_FullBounce_C" (`KismetMathLibrary.MakeTransform` (`self.VBottom`) (struct) (1.0 -1.0 1.0)) "Undefined" "OverrideRootScale")
  (`|SpawnActorFromClass` "/Game/Blueprints/Enemies/BP_Enemy_FullBounce.BP_Enemy_FullBounce_C" (`KismetMathLibrary.MakeTransform` (`self.VCenter`) (struct) (1.0 -1.0 1.0)) "Undefined" "OverrideRootScale")
  (goto _label))

(event `self.ReceiveTick`
  (params (DeltaSeconds :type "Float (single-precision)")))

(event `self.WaveCheck`
  (bind _fright (`self.FRight`))
  (bind _fdepth (`self.FDepth`))
  (bind _fdepth_2 (`self.FDepth`))
  (bind _fright_2 (`self.FRight`))
  (bind _true (`self.CheckWave`))
  (if _true
    (switch `int` (`self.WaveIndex`)
      (:`0`
        (bind _returnvalue (`|SpawnActorFromClass` "/Game/Blueprints/Enemies/BP_Enemy_FlameThrower.BP_Enemy_FlameThrower_C" (`KismetMathLibrary.MakeTransform` (`self.VTop`)) "Undefined" "OverrideRootScale" :!label _label_2))
        (bind _returnvalue_2 (`|SpawnActorFromClass` "/Game/Blueprints/Enemies/BP_Enemy_FlameThrower.BP_Enemy_FlameThrower_C" (`KismetMathLibrary.MakeTransform` (`self.VBottom`)) "Undefined" "OverrideRootScale"))
        (`|ExecutionSequence`
          (:`then_0`
            (bind (_direction _newtrack_0) (`Timeline|Timeline_1` :!label _label_3)
              (:`Update`
                (`self.K2_AddActorLocalOffset` _returnvalue (`KismetMathLibrary.MakeVector` 0.0 0.0 (* _newtrack_0 10.0)) true false)
                (`self.K2_AddActorLocalOffset` _returnvalue_2 (`KismetMathLibrary.MakeVector` 0.0 0.0 (* _newtrack_0 -10.0)) true false))
              (:`Finished`
                (goto _label_3 :!via `PlayFromStart`))))
          (:`then_1`
            (goto _label))))
      (:`1`
        (`|SpawnActorFromClass` "/Game/Blueprints/Enemies/ModularShips/GhostShip/BP_Enemy_GhostShip.BP_Enemy_GhostShip_C" (`KismetMathLibrary.MakeTransform` (`self.VTop`) (struct) (1.0 -1.0 1.0)) "Undefined" "OverrideRootScale" null true true true)
        (`|SpawnActorFromClass` "/Game/Blueprints/Enemies/ModularShips/GhostShip/BP_Enemy_GhostShip.BP_Enemy_GhostShip_C" (`KismetMathLibrary.MakeTransform` (`self.VBottom`) (struct) (1.0 -1.0 1.0)) "Undefined" "OverrideRootScale" null true true true)
        (`|SpawnActorFromClass` "/Game/Blueprints/Enemies/BP_Enemy_ShotGun.BP_Enemy_ShotGun_C" (`KismetMathLibrary.MakeTransform` (`self.VCenter`) (struct) (1.0 -1.0 1.0)) "Undefined" "OverrideRootScale")
        (goto _label))
      (:`2`
        (`|SpawnActorFromClass` "/Game/Blueprints/Enemies/BP_Enemy_FullBounce.BP_Enemy_FullBounce_C" (`KismetMathLibrary.MakeTransform` (`KismetMathLibrary.MakeVector` _fdepth_2 _fright_2) (struct) (1.0 -1.0 1.0)) "Undefined" "OverrideRootScale")
        (`|SpawnActorFromClass` "/Game/Blueprints/Enemies/BP_Enemy_FullBounce.BP_Enemy_FullBounce_C" (`KismetMathLibrary.MakeTransform` (`KismetMathLibrary.MakeVector` _fdepth_2 _fright_2 (/ (`self.FTop`) 2.0))) "Undefined" "OverrideRootScale")
        (`|SpawnActorFromClass` "/Game/Blueprints/Enemies/BP_Enemy_FullBounce.BP_Enemy_FullBounce_C" (`KismetMathLibrary.MakeTransform` (`KismetMathLibrary.MakeVector` _fdepth _fright (/ (`self.FTop`) -2.0))) "Undefined" "OverrideRootScale")
        (`KismetSystemLibrary.Delay` 1.0)
        (`|SpawnActorFromClass` "/Game/Blueprints/Enemies/ModularShips/GhostShip/BP_Enemy_GhostShip.BP_Enemy_GhostShip_C" (`KismetMathLibrary.MakeTransform` (`KismetMathLibrary.MakeVector` _fdepth _fright (/ (`self.FTop`) 4.0))) "Undefined" "OverrideRootScale" null true true)
        (`|SpawnActorFromClass` "/Game/Blueprints/Enemies/ModularShips/GhostShip/BP_Enemy_GhostShip.BP_Enemy_GhostShip_C" (`KismetMathLibrary.MakeTransform` (`KismetMathLibrary.MakeVector` _fdepth _fright (/ (`self.FTop`) -4.0))) "Undefined" "OverrideRootScale" null true true)
        (goto _label))
      (:`3`
        (bind _returnvalue_3 (`|SpawnActorFromClass` "/Game/Blueprints/Enemies/BP_Enemy_Homing.BP_Enemy_Homing_C" (`KismetMathLibrary.MakeTransform` (/ (`self.VTop`) (1.0 1.0 3.0)) (struct) (1.0 -1.0 1.0)) "Undefined" "OverrideRootScale"))
        (bind _returnvalue_4 (`|SpawnActorFromClass` "/Game/Blueprints/Enemies/BP_Enemy_Homing.BP_Enemy_Homing_C" (`KismetMathLibrary.MakeTransform` (/ (`self.VTop`) (1.0 1.0 -3.0)) (struct) (1.0 -1.0 1.0)) "Undefined" "OverrideRootScale"))
        (add `self.OnDestroyed` _returnvalue_4 (delegate `OnDestroyed_Event_0`))
        (add `self.OnDestroyed` _returnvalue_3 (delegate `OnDestroyed_Event_0`)))
      (:`4`
        (`|SpawnActorFromClass` "/Game/Blueprints/Enemies/BP_Enemy_DroneSpawner.BP_Enemy_DroneSpawner_C" (`KismetMathLibrary.MakeTransform` (`self.VCenter`)) "Undefined" "OverrideRootScale")
        (`KismetSystemLibrary.Delay` 1.0)
        (`|SpawnActorFromClass` "/Game/Blueprints/Enemies/BP_Enemy_DroneSpawner.BP_Enemy_DroneSpawner_C" (`KismetMathLibrary.MakeTransform` (`self.VTop`)) "Undefined" "OverrideRootScale")
        (`KismetSystemLibrary.Delay` 1.0)
        (`|SpawnActorFromClass` "/Game/Blueprints/Enemies/BP_Enemy_DroneSpawner.BP_Enemy_DroneSpawner_C" (`KismetMathLibrary.MakeTransform` (`self.VBottom`)) "Undefined" "OverrideRootScale")
        (`KismetSystemLibrary.Delay` 1.0)
        (`|SpawnActorFromClass` "/Game/Blueprints/Enemies/BP_Enemy_FullRotation.BP_Enemy_FullRotation_C" (`KismetMathLibrary.MakeTransform` (/ (`self.VTop`) (1.0 1.0 3.0))) "Undefined" "OverrideRootScale")
        (`KismetSystemLibrary.Delay` 1.0)
        (`|SpawnActorFromClass` "/Game/Blueprints/Enemies/BP_Enemy_FullRotation.BP_Enemy_FullRotation_C" (`KismetMathLibrary.MakeTransform` (/ (`self.VTop`) (1.0 1.0 -3.0))) "Undefined" "OverrideRootScale")
        (goto _label))
      (:`5`
        (goto _label_2))
      (:`6`
        (`|SpawnActorFromClass` "/Game/Blueprints/Enemies/HunterDrone/BP_Enemy_HunterDrone_1_1.BP_Enemy_HunterDrone_1_1_C" (`KismetMathLibrary.MakeTransform` (`self.VCenter`)) "Undefined" "OverrideRootScale")
        (`|SpawnActorFromClass` "/Game/Blueprints/Enemies/HunterDrone/BP_Enemy_HunterDrone_1_1.BP_Enemy_HunterDrone_1_1_C" (`KismetMathLibrary.MakeTransform` (`self.VTop`)) "Undefined" "OverrideRootScale")
        (bind _returnvalue_5 (`|SpawnActorFromClass` "/Game/Blueprints/Enemies/HunterDrone/BP_Enemy_HunterDrone_1_1.BP_Enemy_HunterDrone_1_1_C" (`KismetMathLibrary.MakeTransform` (`self.VBottom`)) "Undefined" "OverrideRootScale"))
        (add `self.OnDestroyed` _returnvalue_5 (delegate `OnDestroyed_Event_3`)))
      (:`7`
        (`|SpawnActorFromClass` "/Game/Blueprints/Enemies/bpEnemyBoss.bpEnemyBoss_C" (`KismetMathLibrary.MakeTransform` (`self.VCenter`)) "Undefined" "OverrideRootScale")
        (goto _label))
      (:`8`
        (bind _returnvalue_6 (`|SpawnActorFromClass` "/Game/Blueprints/Enemies/BP_Enemy_Sling.BP_Enemy_Sling_C" (`KismetMathLibrary.MakeTransform` (`self.VTop`) (struct) (2.0 2.0 2.0)) "Undefined" "OverrideRootScale"))
        (`|ExecutionSequence`
          (:`then_0`
            (bind (_direction_2 _newtrack_0_2) (`Timeline|Timeline_0` :!label _label_4)
              (:`Update`
                (`self.K2_AddActorLocalOffset` _returnvalue_6 (`KismetMathLibrary.MakeVector` 0.0 0.0 (* _newtrack_0_2 50.0)) true false))
              (:`Finished`
                (goto _label_4 :!via `PlayFromStart`))))
          (:`then_1`
            (goto _label))))
      (:`9`
        (bind _returnvalue_7 (`|SpawnActorFromClass` "/Game/Blueprints/Enemies/BP_Enemy_SlingHighFrequency.BP_Enemy_SlingHighFrequency_C" (`KismetMathLibrary.MakeTransform` (`self.VTop`) (struct) (2.0 2.0 2.0)) "Undefined" "OverrideRootScale"))
        (`|ExecutionSequence`
          (:`then_0`
            (bind (_direction_3 _newtrack_0_3) (`Timeline|Timeline_3` :!label _label_5)
              (:`Update`
                (`self.K2_AddActorLocalOffset` _returnvalue_7 (`KismetMathLibrary.MakeVector` 0.0 0.0 (* _newtrack_0_3 50.0)) true false))
              (:`Finished`
                (goto _label_5 :!via `PlayFromStart`))))
          (:`then_1`
            (goto _label))))
      (:`10`
        (bind _returnvalue_8 (`|SpawnActorFromClass` "/Game/Blueprints/Enemies/ModularShips/GhostShip/BP_Enemy_GhostShip.BP_Enemy_GhostShip_C" (`KismetMathLibrary.MakeTransform` (`KismetMathLibrary.MakeVector` (`self.FDepth`) (`self.FRight`)) (struct) (1.0 -1.0 1.0)) "Undefined" "OverrideRootScale"))
        (bind (_returnvalue_x _returnvalue_y _returnvalue_z) (`KismetMathLibrary.BreakVector` (`self.K2_GetActorLocation` _returnvalue_8)))
        (bind _returnvalue_9 (- _returnvalue_y 100.0))
        (`|SpawnActorFromClass` "/Game/Blueprints/Enemies/BP_EnemyTwo.BP_EnemyTwo_C" (`KismetMathLibrary.MakeTransform` (`KismetMathLibrary.MakeVector` _returnvalue_x _returnvalue_9 (+ _returnvalue_z 400.0)) (struct) (1.0 -1.0 1.0)) "Undefined" "OverrideRootScale")
        (`|SpawnActorFromClass` "/Game/Blueprints/Enemies/BP_EnemyTwo.BP_EnemyTwo_C" (`KismetMathLibrary.MakeTransform` (`KismetMathLibrary.MakeVector` _returnvalue_x _returnvalue_9 (- _returnvalue_z 400.0)) (struct) (1.0 -1.0 1.0)) "Undefined" "OverrideRootScale")
        (bind _returnvalue_10 (`|SpawnActorFromClass` "/Game/Blueprints/Enemies/ModularShips/GhostShip/BP_Enemy_GhostShip.BP_Enemy_GhostShip_C" (`KismetMathLibrary.MakeTransform` (`KismetMathLibrary.MakeVector` (`self.FDepth`) (`self.FRight`) (/ (`self.FTop`) 3.0)) (struct) (1.0 -1.0 1.0)) "Undefined" "OverrideRootScale"))
        (bind (_returnvalue_x_2 _returnvalue_y_2 _returnvalue_z_2) (`KismetMathLibrary.BreakVector` (`self.K2_GetActorLocation` _returnvalue_10)))
        (bind _returnvalue_11 (- _returnvalue_y_2 100.0))
        (`|SpawnActorFromClass` "/Game/Blueprints/Enemies/BP_EnemyTwo.BP_EnemyTwo_C" (`KismetMathLibrary.MakeTransform` (`KismetMathLibrary.MakeVector` _returnvalue_x_2 _returnvalue_11 (+ _returnvalue_z_2 400.0)) (struct) (1.0 -1.0 1.0)) "Undefined" "OverrideRootScale")
        (`|SpawnActorFromClass` "/Game/Blueprints/Enemies/BP_EnemyTwo.BP_EnemyTwo_C" (`KismetMathLibrary.MakeTransform` (`KismetMathLibrary.MakeVector` _returnvalue_x_2 _returnvalue_11 (- _returnvalue_z_2 400.0)) (struct) (1.0 -1.0 1.0)) "Undefined" "OverrideRootScale")
        (bind _returnvalue_12 (`|SpawnActorFromClass` "/Game/Blueprints/Enemies/ModularShips/GhostShip/BP_Enemy_GhostShip.BP_Enemy_GhostShip_C" (`KismetMathLibrary.MakeTransform` (`KismetMathLibrary.MakeVector` (`self.FDepth`) (`self.FRight`) (/ (`self.FTop`) -3.0)) (struct) (1.0 -1.0 1.0)) "Undefined" "OverrideRootScale"))
        (bind (_returnvalue_x_3 _returnvalue_y_3 _returnvalue_z_3) (`KismetMathLibrary.BreakVector` (`self.K2_GetActorLocation` _returnvalue_12)))
        (bind _returnvalue_13 (- _returnvalue_y_3 100.0))
        (`|SpawnActorFromClass` "/Game/Blueprints/Enemies/BP_EnemyTwo.BP_EnemyTwo_C" (`KismetMathLibrary.MakeTransform` (`KismetMathLibrary.MakeVector` _returnvalue_x_3 _returnvalue_13 (+ _returnvalue_z_3 400.0)) (struct) (1.0 -1.0 1.0)) "Undefined" "OverrideRootScale")
        (`|SpawnActorFromClass` "/Game/Blueprints/Enemies/BP_EnemyTwo.BP_EnemyTwo_C" (`KismetMathLibrary.MakeTransform` (`KismetMathLibrary.MakeVector` _returnvalue_x_3 _returnvalue_13 (- _returnvalue_z_3 400.0)) (struct) (1.0 -1.0 1.0)) "Undefined" "OverrideRootScale")
        (goto _label))
      (:`11`
        (bind _returnvalue_14 (`|SpawnActorFromClass` "/Game/Blueprints/Enemies/BP_Enemy_Sling.BP_Enemy_Sling_C" (`KismetMathLibrary.MakeTransform` (`self.VTop`)) "Undefined" "OverrideRootScale"))
        (bind _returnvalue_15 (`|SpawnActorFromClass` "/Game/Blueprints/Enemies/BP_Enemy_Sling.BP_Enemy_Sling_C" (`KismetMathLibrary.MakeTransform` (`self.VBottom`)) "Undefined" "OverrideRootScale"))
        (`|ExecutionSequence`
          (:`then_0`
            (bind (_direction_4 _newtrack_0_4) (`Timeline|Timeline_4` :!label _label_6)
              (:`Update`
                (`self.K2_AddActorLocalOffset` _returnvalue_14 (`KismetMathLibrary.MakeVector` 0.0 0.0 (* _newtrack_0_4 10.0)) true false)
                (`self.K2_AddActorLocalOffset` _returnvalue_15 (`KismetMathLibrary.MakeVector` 0.0 0.0 (* _newtrack_0_4 -10.0)) true false))
              (:`Finished`
                (goto _label_6 :!via `PlayFromStart`))))
          (:`then_1`
            (goto _label)))))))

(event `OnDestroyed_Event_3` :!signature `self.OnDestroyed`
  (params (DestroyedActor :type "Actor Object Reference"))
  (`|SpawnActorFromClass` "/Game/Blueprints/Enemies/HunterDrone/BP_Enemy_HunterDrone_1_2_1.BP_Enemy_HunterDrone_1_2_1_C" (`KismetMathLibrary.MakeTransform` (`self.VCenter`)) "Undefined" "OverrideRootScale")
  (`|SpawnActorFromClass` "/Game/Blueprints/Enemies/HunterDrone/BP_Enemy_HunterDrone_1_2_1.BP_Enemy_HunterDrone_1_2_1_C" (`KismetMathLibrary.MakeTransform` (`self.VTop`)) "Undefined" "OverrideRootScale")
  (`|SpawnActorFromClass` "/Game/Blueprints/Enemies/HunterDrone/BP_Enemy_HunterDrone_1_2_1.BP_Enemy_HunterDrone_1_2_1_C" (`KismetMathLibrary.MakeTransform` (`self.VBottom`)) "Undefined" "OverrideRootScale")
  (goto _label))

(fn `UserConstructionScript`
  (`parent.UserConstructionScript`))