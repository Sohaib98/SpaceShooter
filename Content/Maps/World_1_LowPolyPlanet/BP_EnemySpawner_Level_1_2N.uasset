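; Enemy spawner for World 1 (LowPolyPlanet) that runs a scripted ten-wave level, ending with two scaled-down bosses.
; When CheckWave passes, WaveCheck switches on WaveIndex to a collapsed graph per wave, then increments it, or calls the game mode's AllEnemiesDefeated after the last.
; Waves place ghost ships, drones and other enemies relative to edge and center variables, some staggered by delays.
; The ninth wave moves an enlarged drone with a looping Timeline.
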(event `self.ReceiveTick`
  (params (DeltaSeconds :type "Float (single-precision)")))

(event `self.WaveCheck`
  (bind _fright (`self.FRight`))
  (bind _fdepth (`self.FDepth`))
  (bind _fdepth_2 (`self.FDepth`))
  (bind _fright_2 (`self.FRight`))
  (bind (_vcenter_x _vcenter_y _vcenter_z) (`KismetMathLibrary.BreakVector` (`self.VCenter`)))
  (bind (_vcenter_x_2 _vcenter_y_2 _vcenter_z_2) (`KismetMathLibrary.BreakVector` (`self.VCenter`)))
  (bind (_vcenter_x_3 _vcenter_y_3 _vcenter_z_3) (`KismetMathLibrary.BreakVector` (`self.VCenter`)))
  (bind (_vcenter_x_4 _vcenter_y_4 _vcenter_z_4) (`KismetMathLibrary.BreakVector` (`self.VCenter`)))
  (bind (_vcenter_x_5 _vcenter_y_5 _vcenter_z_5) (`KismetMathLibrary.BreakVector` (`self.VCenter`)))
  (bind (_vcenter_x_6 _vcenter_y_6 _vcenter_z_6) (`KismetMathLibrary.BreakVector` (`self.VCenter`)))
  (bind _returnvalue (/ (`self.FTop`) 2.0))
  (bind _true (`self.CheckWave`))
  (if _true
    (switch `int` (`self.WaveIndex`)
      (:`Default`
        (`/Game/Blueprints/Misc/bpGameMode.AllEnemiesDefeated` (`self.bpGameMode`) "/Game/Blueprints/UI/QuitMenu.QuitMenu_C"))
      (:`0`
        (`|SpawnActorFromClass` "/Game/Blueprints/Enemies/ModularShips/GhostShip/BP_Enemy_GhostShip.BP_Enemy_GhostShip_C" (`KismetMathLibrary.MakeTransform` (`KismetMathLibrary.MakeVector` (`self.FDepth`) (`self.FRight`)) (struct) (1.0 -1.0 1.0)) "Undefined" "OverrideRootScale")
        (`self.IncrementWave` :!label _label))
      (:`1`
        (`|SpawnActorFromClass` "/Game/Blueprints/Enemies/ModularShips/GhostShip/BP_Enemy_GhostShip.BP_Enemy_GhostShip_C" (`KismetMathLibrary.MakeTransform` (`KismetMathLibrary.MakeVector` (`self.FDepth`) (`self.FRight`)) (struct) (1.0 -1.0 1.0)) "Undefined" "OverrideRootScale")
        (`KismetSystemLibrary.Delay` 1.0)
        (`|SpawnActorFromClass` "/Game/Blueprints/Enemies/ModularShips/GhostShip/BP_Enemy_GhostShip.BP_Enemy_GhostShip_C" (`KismetMathLibrary.MakeTransform` (`KismetMathLibrary.MakeVector` (`self.FDepth`) (`self.FRight`) _returnvalue) (struct) (1.0 -1.0 1.0)) "Undefined" "OverrideRootScale")
        (`|SpawnActorFromClass` "/Game/Blueprints/Enemies/ModularShips/GhostShip/BP_Enemy_GhostShip.BP_Enemy_GhostShip_C" (`KismetMathLibrary.MakeTransform` (`KismetMathLibrary.MakeVector` (`self.FDepth`) (`self.FRight`) (* _returnvalue -1.0)) (struct) (1.0 -1.0 1.0)) "Undefined" "OverrideRootScale")
        (goto _label))
      (:`2`
        (`|SpawnActorFromClass` "/Game/Blueprints/Enemies/ModularShips/GhostShip/BP_Enemy_GhostShip.BP_Enemy_GhostShip_C" (`KismetMathLibrary.MakeTransform` (`KismetMathLibrary.MakeVector` _fdepth_2 _fright_2) (struct) (1.0 -1.0 1.0)) "Undefined" "OverrideRootScale")
        (`|SpawnActorFromClass` "/Game/Blueprints/Enemies/BP_EnemyTwo.BP_EnemyTwo_C" (`KismetMathLibrary.MakeTransform` (`KismetMathLibrary.MakeVector` _fdepth_2 _fright_2 (/ (`self.FTop`) 2.0))) "Undefined" "OverrideRootScale")
        (`|SpawnActorFromClass` "/Game/Blueprints/Enemies/BP_EnemyTwo.BP_EnemyTwo_C" (`KismetMathLibrary.MakeTransform` (`KismetMathLibrary.MakeVector` _fdepth _fright (/ (`self.FTop`) -2.0))) "Undefined" "OverrideRootScale")
        (`KismetSystemLibrary.Delay` 1.0)
        (`|SpawnActorFromClass` "/Game/Blueprints/Enemies/BP_EnemyTwo.BP_EnemyTwo_C" (`KismetMathLibrary.MakeTransform` (`KismetMathLibrary.MakeVector` _fdepth _fright (/ (`self.FTop`) 4.0))) "Undefined" "OverrideRootScale")
        (`|SpawnActorFromClass` "/Game/Blueprints/Enemies/BP_EnemyTwo.BP_EnemyTwo_C" (`KismetMathLibrary.MakeTransform` (`KismetMathLibrary.MakeVector` _fdepth _fright (/ (`self.FTop`) -4.0))) "Undefined" "OverrideRootScale")
        (goto _label))
      (:`3`
        (`|SpawnActorFromClass` "/Game/Blueprints/Enemies/ModularShips/GhostShip/BP_Enemy_GhostShip.BP_Enemy_GhostShip_C" (`KismetMathLibrary.MakeTransform` (`KismetMathLibrary.MakeVector` (`self.FDepth`) (`self.FRight`)) (struct) (1.0 -1.0 1.0)) "Undefined" "OverrideRootScale")
        (`|SpawnActorFromClass` "/Game/Blueprints/Enemies/ModularShips/GhostShip/BP_Enemy_GhostShip.BP_Enemy_GhostShip_C" (`KismetMathLibrary.MakeTransform` (`KismetMathLibrary.MakeVector` (`self.FDepth`) (- (`self.FRight`) 300.0) (- (`self.FTop`) 50.0)) (struct) (1.0 -1.0 1.0)) "Undefined" "OverrideRootScale")
        (`|SpawnActorFromClass` "/Game/Blueprints/Enemies/ModularShips/GhostShip/BP_Enemy_GhostShip.BP_Enemy_GhostShip_C" (`KismetMathLibrary.MakeTransform` (`KismetMathLibrary.MakeVector` (`self.FDepth`) (- (`self.FRight`) 300.0) (- (`self.FTop`) -50.0)) (struct) (1.0 -1.0 1.0)) "Undefined" "OverrideRootScale")
        (`|SpawnActorFromClass` "/Game/Blueprints/Enemies/ModularShips/GhostShip/BP_Enemy_GhostShip.BP_Enemy_GhostShip_C" (`KismetMathLibrary.MakeTransform` (`KismetMathLibrary.MakeVector` (`self.FDepth`) (`self.FRight`) (/ (`self.FTop`) 2.0)) (struct) (1.0 -1.0 1.0)) "Undefined" "OverrideRootScale")
        (`|SpawnActorFromClass` "/Game/Blueprints/Enemies/ModularShips/GhostShip/BP_Enemy_GhostShip.BP_Enemy_GhostShip_C" (`KismetMathLibrary.MakeTransform` (`KismetMathLibrary.MakeVector` (`self.FDepth`) (- (`self.FRight`) 300.0) (- (/ (`self.FTop`) 2.0) 50.0)) (struct) (1.0 -1.0 1.0)) "Undefined" "OverrideRootScale")
        (`|SpawnActorFromClass` "/Game/Blueprints/Enemies/ModularShips/GhostShip/BP_Enemy_GhostShip.BP_Enemy_GhostShip_C" (`KismetMathLibrary.MakeTransform` (`KismetMathLibrary.MakeVector` (`self.FDepth`) (- (`self.FRight`) 300.0) (- (/ (`self.FTop`) 2.0) -50.0)) (struct) (1.0 -1.0 1.0)) "Undefined" "OverrideRootScale")
        (goto _label))
      (:`4`
        (`|SpawnActorFromClass` "/Game/Blueprints/Enemies/HunterDrone/BP_Enemy_HunterDrone_2_2_2.BP_Enemy_HunterDrone_2_2_2_C" (`KismetMathLibrary.MakeTransform` (`self.VCenter`)) "Undefined" "OverrideRootScale")
        (goto _label))
      (:`5`
        (`|SpawnActorFromClass` "/Game/Blueprints/Enemies/HunterDrone/BP_Enemy_HunterDrone_2_2_2.BP_Enemy_HunterDrone_2_2_2_C" (`KismetMathLibrary.MakeTransform` (`self.VTop`)) "Undefined" "OverrideRootScale")
        (`|SpawnActorFromClass` "/Game/Blueprints/Enemies/HunterDrone/BP_Enemy_HunterDrone_2_2_2.BP_Enemy_HunterDrone_2_2_2_C" (`KismetMathLibrary.MakeTransform` (`self.VBottom`)) "Undefined" "OverrideRootScale")
        (goto _label))
      (:`6`
        (`|SpawnActorFromClass` "/Game/Blueprints/Enemies/BP_EnemyTwo.BP_EnemyTwo_C" (`KismetMathLibrary.MakeTransform` (`self.VCenter`)) "Undefined" "OverrideRootScale")
        (`KismetSystemLibrary.Delay` 1.0)
        (`|SpawnActorFromClass` "/Game/Blueprints/Enemies/HunterDrone/BP_Enemy_HunterDrone_2_2_2.BP_Enemy_HunterDrone_2_2_2_C" (`KismetMathLibrary.MakeTransform` (`self.VTop`)) "Undefined" "OverrideRootScale")
        (`|SpawnActorFromClass` "/Game/Blueprints/Enemies/HunterDrone/BP_Enemy_HunterDrone_2_2_2.BP_Enemy_HunterDrone_2_2_2_C" (`KismetMathLibrary.MakeTransform` (`self.VBottom`)) "Undefined" "OverrideRootScale")
        (goto _label))
      (:`7`
        (`|SpawnActorFromClass` "/Game/Blueprints/Enemies/HunterDrone/BP_Enemy_HunterDrone_2_2_2.BP_Enemy_HunterDrone_2_2_2_C" (`KismetMathLibrary.MakeTransform` (`self.VCenter`)) "Undefined" "OverrideRootScale")
        (`|SpawnActorFromClass` "/Game/Blueprints/Enemies/ModularShips/GhostShip/BP_Enemy_GhostShip.BP_Enemy_GhostShip_C" (`KismetMathLibrary.MakeTransform` (`KismetMathLibrary.MakeVector` _vcenter_x_2 _vcenter_y_2 (+ _vcenter_z_2 200.0)) (struct) (1.0 -1.0 1.0)) "Undefined" "OverrideRootScale")
        (`|SpawnActorFromClass` "/Game/Blueprints/Enemies/ModularShips/GhostShip/BP_Enemy_GhostShip.BP_Enemy_GhostShip_C" (`KismetMathLibrary.MakeTransform` (`KismetMathLibrary.MakeVector` _vcenter_x_3 _vcenter_y_3 (+ _vcenter_z_3 -200.0)) (struct) (1.0 -1.0 1.0)) "Undefined" "OverrideRootScale")
        (`|SpawnActorFromClass` "/Game/Blueprints/Enemies/BP_EnemyTwo.BP_EnemyTwo_C" (`KismetMathLibrary.MakeTransform` (`KismetMathLibrary.MakeVector` _vcenter_x_4 _vcenter_y_4 (+ _vcenter_z_4 -400.0))) "Undefined" "OverrideRootScale")
        (`|SpawnActorFromClass` "/Game/Blueprints/Enemies/BP_EnemyTwo.BP_EnemyTwo_C" (`KismetMathLibrary.MakeTransform` (`KismetMathLibrary.MakeVector` _vcenter_x_5 _vcenter_y_5 (+ _vcenter_z_5 400.0))) "Undefined" "OverrideRootScale")
        (`|SpawnActorFromClass` "/Game/Blueprints/Enemies/bpEnemyOne.bpEnemyOne_C" (`KismetMathLibrary.MakeTransform` (`KismetMathLibrary.MakeVector` _vcenter_x_6 _vcenter_y_6 (+ _vcenter_z_6 600.0))) "Undefined" "OverrideRootScale")
        (`|SpawnActorFromClass` "/Game/Blueprints/Enemies/bpEnemyOne.bpEnemyOne_C" (`KismetMathLibrary.MakeTransform` (`KismetMathLibrary.MakeVector` _vcenter_x _vcenter_y (+ _vcenter_z -600.0))) "Undefined" "OverrideRootScale")
        (goto _label))
      (:`8`
        (bind _returnvalue_2 (`|SpawnActorFromClass` "/Game/Blueprints/Enemies/HunterDrone/BP_Enemy_HunterDrone_2_2_2.BP_Enemy_HunterDrone_2_2_2_C" (`KismetMathLibrary.MakeTransform` (`self.VTop`) (struct) (2.0 2.0 2.0)) "Undefined" "OverrideRootScale"))
        (`|ExecutionSequence`
          (:`then_0`
            (bind (_direction _newtrack_0) (`Timeline|Timeline_0` :!label _label_2)
              (:`Update`
                (`self.K2_AddActorLocalOffset` _returnvalue_2 (`KismetMathLibrary.MakeVector` 0.0 0.0 (* _newtrack_0 50.0)) true false))
              (:`Finished`
                (goto _label_2 :!via `PlayFromStart`))))
          (:`then_1`
            (goto _label))))
      (:`9`
        (`|SpawnActorFromClass` "/Game/Blueprints/Enemies/bpEnemyBoss.bpEnemyBoss_C" (`KismetMathLibrary.MakeTransform` (`self.VTop`) (struct) (0.5 0.5 0.5)) "Undefined" "OverrideRootScale")
        (`|SpawnActorFromClass` "/Game/Blueprints/Enemies/bpEnemyBoss.bpEnemyBoss_C" (`KismetMathLibrary.MakeTransform` (`self.VBottom`) (struct) (0.5 0.5 0.5)) "Undefined" "OverrideRootScale")
        (goto _label)))))

(fn `UserConstructionScript`
  (`parent.UserConstructionScript`))