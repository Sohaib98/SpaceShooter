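; Touch-driven planet selector that swaps the active level actor when one of five planet collisions is tapped.
; Each tap runs its own copy of the same collapsed graph, skipping the already active class and disabling touch events during the swap.
; Timelines scale the current level and BP_Sky_Sphere actors to zero before destruction, then grow the newly spawned, zero-scale level and sky spheres in.
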(event `self.ReceiveBeginPlay`
  (set `PlayerController.bEnableTouchEvents` true (`GameplayStatics.GetPlayerController` 0)))

(event `self.Planet_1_Collision.OnInputTouchBegin`
  (params (FingerIndex :type "ETouchIndex Enum" :default "Touch1") (TouchedComponent :type "PrimitiveComponent Object Reference"))
  (bind _output (`|GetArrayItem` (`self.LevelsToBeSpawned`)))
  (if (!= (`GameplayStatics.GetObjectClass` (`self.ActivePlanet`)) _output)
    (set `PlayerController.bEnableTouchEvents` false (`GameplayStatics.GetPlayerController` 0))
    (`/Engine/EditorBlueprintResources/StandardMacros.IsValid` (`self.ActivePlanet`)
      (:`Is Valid`
        (bind (_direction _newtrack_4) (`Timeline|Timeline_0` :!via `PlayFromStart`)
          (:`Update`
            (bind (_leveltobedestroyed _skyboxtobedestoryed) (`self.TransitionOut` (`self.ActivePlanet`) _newtrack_4))
            (`KismetSystemLibrary.Delay` 5.0))
          (:`Finished`
            (`self.K2_DestroyActor` _skyboxtobedestoryed)
            (`self.K2_DestroyActor` _leveltobedestroyed)
            (bind _spawnedlevel (`self.SpawnLevel` _output :!label _label))
            (bind _output_get (set `self.ActivePlanet` _spawnedlevel))
            (bind (_direction_2 _newtrack_0) (`Timeline|Timeline_1` :!via `PlayFromStart`)
              (:`Update`
                (`self.TransitionIn` _output_get _newtrack_0)
                (`KismetSystemLibrary.Delay` 1.0)
                (set `PlayerController.bEnableTouchEvents` true (`GameplayStatics.GetPlayerController` 0)))))))
      (:`Is Not Valid`
        (goto _label)))))

(event `self.Planet_2_Collision.OnInputTouchBegin`
  (params (FingerIndex :type "ETouchIndex Enum" :default "Touch1") (TouchedComponent :type "PrimitiveComponent Object Reference"))
  (bind _output (`|GetArrayItem` (`self.LevelsToBeSpawned`) 1))
  (if (!= (`GameplayStatics.GetObjectClass` (`self.ActivePlanet`)) _output)
    (set `PlayerController.bEnableTouchEvents` false (`GameplayStatics.GetPlayerController` 0))
    (`/Engine/EditorBlueprintResources/StandardMacros.IsValid` (`self.ActivePlanet`)
      (:`Is Valid`
        (bind (_direction _newtrack_4) (`Timeline|Timeline_3` :!via `PlayFromStart`)
          (:`Update`
            (bind (_leveltobedestroyed _skyboxtobedestoryed) (`self.TransitionOut` (`self.ActivePlanet`) _newtrack_4))
            (`KismetSystemLibrary.Delay` 5.0))
          (:`Finished`
            (`self.K2_DestroyActor` _skyboxtobedestoryed)
            (`self.K2_DestroyActor` _leveltobedestroyed)
            (bind _spawnedlevel (`self.SpawnLevel` _output :!label _label_2))
            (bind _output_get (set `self.ActivePlanet` _spawnedlevel))
            (bind (_direction_2 _newtrack_0) (`Timeline|Timeline_2` :!via `PlayFromStart`)
              (:`Update`
                (`self.TransitionIn` _output_get _newtrack_0)
                (`KismetSystemLibrary.Delay` 1.0)
                (set `PlayerController.bEnableTouchEvents` true (`GameplayStatics.GetPlayerController` 0)))))))
      (:`Is Not Valid`
        (goto _label_2)))))

(event `self.Planet_3_Collision.OnInputTouchBegin`
  (params (FingerIndex :type "ETouchIndex Enum" :default "Touch1") (TouchedComponent :type "PrimitiveComponent Object Reference"))
  (bind _output (`|GetArrayItem` (`self.LevelsToBeSpawned`) 2))
  (if (!= (`GameplayStatics.GetObjectClass` (`self.ActivePlanet`)) _output)
    (set `PlayerController.bEnableTouchEvents` false (`GameplayStatics.GetPlayerController` 0))
    (`/Engine/EditorBlueprintResources/StandardMacros.IsValid` (`self.ActivePlanet`)
      (:`Is Valid`
        (bind (_direction _newtrack_4) (`Timeline|Timeline_5` :!via `PlayFromStart`)
          (:`Update`
            (bind (_leveltobedestroyed _skyboxtobedestoryed) (`self.TransitionOut` (`self.ActivePlanet`) _newtrack_4))
            (`KismetSystemLibrary.Delay` 5.0))
          (:`Finished`
            (`self.K2_DestroyActor` _skyboxtobedestoryed)
            (`self.K2_DestroyActor` _leveltobedestroyed)
            (bind _spawnedlevel (`self.SpawnLevel` _output :!label _label_3))
            (bind _output_get (set `self.ActivePlanet` _spawnedlevel))
            (bind (_direction_2 _newtrack_0) (`Timeline|Timeline_4` :!via `PlayFromStart`)
              (:`Update`
                (`self.TransitionIn` _output_get _newtrack_0)
                (`KismetSystemLibrary.Delay` 1.0)
                (set `PlayerController.bEnableTouchEvents` true (`GameplayStatics.GetPlayerController` 0)))))))
      (:`Is Not Valid`
        (goto _label_3)))))

(event `self.Planet_4_Collision.OnInputTouchBegin`
  (params (FingerIndex :type "ETouchIndex Enum" :default "Touch1") (TouchedComponent :type "PrimitiveComponent Object Reference"))
  (bind _output (`|GetArrayItem` (`self.LevelsToBeSpawned`) 3))
  (if (!= (`GameplayStatics.GetObjectClass` (`self.ActivePlanet`)) _output)
    (set `PlayerController.bEnableTouchEvents` false (`GameplayStatics.GetPlayerController` 0))
    (`/Engine/EditorBlueprintResources/StandardMacros.IsValid` (`self.ActivePlanet`)
      (:`Is Valid`
        (bind (_direction _newtrack_4) (`Timeline|Timeline_7` :!via `PlayFromStart`)
          (:`Update`
            (bind (_leveltobedestroyed _skyboxtobedestoryed) (`self.TransitionOut` (`self.ActivePlanet`) _newtrack_4))
            (`KismetSystemLibrary.Delay` 5.0))
          (:`Finished`
            (`self.K2_DestroyActor` _skyboxtobedestoryed)
            (`self.K2_DestroyActor` _leveltobedestroyed)
            (bind _spawnedlevel (`self.SpawnLevel` _output :!label _label_4))
            (bind _output_get (set `self.ActivePlanet` _spawnedlevel))
            (bind (_direction_2 _newtrack_0) (`Timeline|Timeline_6` :!via `PlayFromStart`)
              (:`Update`
                (`self.TransitionIn` _output_get _newtrack_0)
                (`KismetSystemLibrary.Delay` 1.0)
                (set `PlayerController.bEnableTouchEvents` true (`GameplayStatics.GetPlayerController` 0)))))))
      (:`Is Not Valid`
        (goto _label_4)))))

(event `self.Planet_5_Collision.OnInputTouchBegin`
  (params (FingerIndex :type "ETouchIndex Enum" :default "Touch1") (TouchedComponent :type "PrimitiveComponent Object Reference"))
  (bind _output (`|GetArrayItem` (`self.LevelsToBeSpawned`) 4))
  (if (!= (`GameplayStatics.GetObjectClass` (`self.ActivePlanet`)) _output)
    (set `PlayerController.bEnableTouchEvents` false (`GameplayStatics.GetPlayerController` 0))
    (`/Engine/EditorBlueprintResources/StandardMacros.IsValid` (`self.ActivePlanet`)
      (:`Is Valid`
        (bind (_direction _newtrack_4) (`Timeline|Timeline_11` :!via `PlayFromStart`)
          (:`Update`
            (bind (_leveltobedestroyed _skyboxtobedestoryed) (`self.TransitionOut` (`self.ActivePlanet`) _newtrack_4))
            (`KismetSystemLibrary.Delay` 5.0))
          (:`Finished`
            (`self.K2_DestroyActor` _skyboxtobedestoryed)
            (`self.K2_DestroyActor` _leveltobedestroyed)
            (bind _spawnedlevel (`self.SpawnLevel` _output :!label _label_5))
            (bind _output_get (set `self.ActivePlanet` _spawnedlevel))
            (bind (_direction_2 _newtrack_0) (`Timeline|Timeline_10` :!via `PlayFromStart`)
              (:`Update`
                (`self.TransitionIn` _output_get _newtrack_0)
                (`KismetSystemLibrary.Delay` 1.0)
                (set `PlayerController.bEnableTouchEvents` true (`GameplayStatics.GetPlayerController` 0)))))))
      (:`Is Not Valid`
        (goto _label_5)))))

(fn `SpawnLevel`
  (params (LevelToBeSpawned :type "Actor Class Reference"))
  (returns (SpawnedLevel :type "Actor Object Reference"))
  (bind _returnvalue (`|SpawnActorFromClass` LevelToBeSpawned (`KismetMathLibrary.MakeTransform` (0.0 0.0 0.0) (struct) (0.0 0.0 0.0)) "Undefined" "OverrideRootScale"))
  (return _returnvalue))

(fn `TransitionIn`
  (params (LevelToBeTransitionedIn :type "Actor Object Reference") (TimeLine :type "Float (double-precision)"))
  (`self.SetActorScale3D` LevelToBeTransitionedIn (`KismetMathLibrary.VLerp` (`self.GetActorScale3D` LevelToBeTransitionedIn) (1.0 1.0 1.0) TimeLine))
  (bind _outactors (`GameplayStatics.GetAllActorsOfClass` "/Engine/EngineSky/BP_Sky_Sphere.BP_Sky_Sphere_C"))
  (for _array_element _outactors
    (`self.SetActorScale3D` _array_element (`KismetMathLibrary.VLerp` (`self.GetActorScale3D` _array_element) (0.1 0.1 0.1) TimeLine))))

(fn `TransitionOut`
  (params (LevelToBeTransitionedOut :type "Actor Object Reference") (TimeLine :type "Float (double-precision)"))
  (returns (LevelToBeDestroyed :type "Actor Object Reference") (SkyBoxToBeDestoryed :type "Actor Object Reference"))
  (`self.SetActorScale3D` LevelToBeTransitionedOut (`KismetMathLibrary.VLerp` (`self.GetActorScale3D` LevelToBeTransitionedOut) (0.0 0.0 0.0) TimeLine))
  (bind _outactors (`GameplayStatics.GetAllActorsOfClass` "/Engine/EngineSky/BP_Sky_Sphere.BP_Sky_Sphere_C"))
  (for _array_element _outactors
    (`self.SetActorScale3D` _array_element (`KismetMathLibrary.VLerp` (`self.GetActorScale3D` _array_element) (0.0 0.0 0.0) TimeLine))
    (return LevelToBeTransitionedOut _array_element)))

(fn `UserConstructionScript`)