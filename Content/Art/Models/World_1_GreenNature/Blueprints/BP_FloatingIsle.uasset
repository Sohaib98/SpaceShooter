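; Floating island actor for the green nature world that drifts, spins and hovers.
; The construction script randomly places tree meshes at four marker components, with random yaw and uniform scale.
; BeginPlay picks random spin and speed, which Tick applies as per-frame yaw and world Y steps, unscaled by delta time.
; A Hover timeline lerps height toward 500 units below the start, replaying in reverse from the end whenever it finishes.
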(event `self.ReceiveBeginPlay`
  (bind (_returnvalue_x _returnvalue_y _returnvalue_z) (`KismetMathLibrary.BreakVector` (`self.K2_GetActorLocation`)))
  (bind (_returnvalue_x_2 _returnvalue_y_2) (`KismetMathLibrary.BreakVector` (`self.K2_GetActorLocation`)))
  (set `self.FRandomRotation` (`KismetMathLibrary.RandomFloatInRange` -0.25 0.25))
  (bind _output_get (set `self.FMoveSpeed` (`KismetMathLibrary.RandomFloatInRange` (`self.FMinMoveSpeed`) (`self.FMaxMoveSpeed`))))
  (set `self.FActorZ` _returnvalue_z)
  (bind (_direction _newtrack_0) (`Timeline|Timeline_0` :!via `PlayFromStart` :!label _label)
    (:`Update`
      (`self.K2_SetActorLocation` (`KismetMathLibrary.MakeVector` _returnvalue_x_2 _returnvalue_y_2 (`KismetMathLibrary.Lerp` (+ (`self.FActorZ`) 0.0) (- (`self.FActorZ`) 500.0) _newtrack_0))))
    (:`Finished`
      (goto _label :!via `ReverseFromEnd`))))

(event `self.ReceiveTick`
  (params (DeltaSeconds :type "Float (single-precision)"))
  (bind (_returnvalue_roll _returnvalue_pitch _returnvalue_yaw) (`KismetMathLibrary.BreakRotator` (`self.K2_GetActorRotation`)))
  (bind (_returnvalue_x _returnvalue_y _returnvalue_z) (`KismetMathLibrary.BreakVector` (`self.K2_GetActorLocation`)))
  (`self.K2_SetActorRotation` (`KismetMathLibrary.MakeRotator` 0.0 0.0 (+ _returnvalue_yaw (`self.FRandomRotation`))))
  (`self.K2_SetActorLocation` (`KismetMathLibrary.MakeVector` _returnvalue_x (+ _returnvalue_y (stale `self.ReceiveBeginPlay` _output_get)) _returnvalue_z)))

(fn `SetSpawnPoints`
  (set `self.TreeSpawnLocations` (`|MakeArray` (`SceneComponent.GetRelativeTransform` (`self.1`)) (`SceneComponent.GetRelativeTransform` (`self.2`)) (`SceneComponent.GetRelativeTransform` (`self.3`)) (`SceneComponent.GetRelativeTransform` (`self.4`)))))

(fn `SpawnTrees`
  (bind _treemeshes (`self.TreeMeshes`))
  (for _array_element (`self.TreeSpawnLocations`)
    (if (`KismetMathLibrary.RandomBool`)
      (bind _returnvalue (`AddComponent|NODE_AddStaticMeshComponent-1` :`RelativeTransform` (`KismetMathLibrary.MakeTransform` (.location _array_element) (`KismetMathLibrary.MakeRotator` (.roll (.rotation _array_element)) (.pitch (.rotation _array_element)) (`KismetMathLibrary.RandomFloatInRange` 0.0 180.0)) (`KismetMathLibrary.Conv_DoubleToVector` (`KismetMathLibrary.RandomFloatInRange` 0.5 2.0)))))
      (`StaticMeshComponent.SetStaticMesh` _returnvalue (`|GetArrayItem` _treemeshes (`KismetMathLibrary.RandomIntegerInRange` 0 (`KismetArrayLibrary.Array_LastIndex` _treemeshes)))))))

(fn `UserConstructionScript`
  (`self.SetSpawnPoints`)
  (`self.SpawnTrees`))