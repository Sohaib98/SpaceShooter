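; Spawner actor that populates the green nature world with floating isles, creating one on BeginPlay and more at a set interval through a Delay on Tick.
; Each spawn gets random X, Z, yaw and uniform scale within configurable ranges.
; Its Y position adds the viewport height, the random X and a multiple of the stored isle reference's bounds extent, apparently to offset it out of view.
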(event `self.ReceiveBeginPlay`
  (bind _transform (`self.GetRandomTransform`))
  (bind _returnvalue (`|SpawnActorFromClass` (`self.Isle`) _transform "Undefined" "OverrideRootScale"))
  (set `self.IsleRef` _returnvalue :!label _label))

(event `self.ReceiveTick`
  (params (DeltaSeconds :type "Float (single-precision)"))
  (`KismetSystemLibrary.Delay` (`self.SpawnInterval`))
  (bind _transform (`self.GetRandomTransform`))
  (`|SpawnActorFromClass` (`self.Isle`) _transform "Undefined" "OverrideRootScale")
  (goto _label))

(fn `GetRandomScale`
  (returns (RandomScale :type "Float (double-precision)"))
  (return (`KismetMathLibrary.RandomFloatInRange` (`self.FMinScale`) (`self.FMaxScale`))))

(fn `GetRandomTransform`
  (returns (Transform :type "Transform Structure"))
  (bind (_returnvalue_x _returnvalue_y) (`KismetMathLibrary.BreakVector2D` (`WidgetLayoutLibrary.GetViewportSize`)))
  (bind _randomx (`self.GetRandomX`))
  (bind _randomz (`self.GetRandomZ`))
  (bind _randomscale (`self.GetRandomScale`))
  (return (`KismetMathLibrary.MakeTransform` (`KismetMathLibrary.MakeVector` _randomx (+ _returnvalue_y _randomx (* (.y (`.BoxExtent` (`self.GetActorBounds` (`self.IsleRef`) false))) 4.0)) _randomz) (`KismetMathLibrary.MakeRotator` 0.0 0.0 (`KismetMathLibrary.RandomFloatInRange` (`self.FIsleMinRotation`) (`self.FIsleMaxRotation`))) (`KismetMathLibrary.Conv_DoubleToVector` _randomscale))))

(fn `GetRandomX`
  (returns (RandomX :type "Float (double-precision)"))
  (return (`KismetMathLibrary.RandomFloatInRange` (`self.FMinX`) (`self.FMaxX`))))

(fn `GetRandomZ`
  (returns (RandomZ :type "Float (double-precision)"))
  (return (`KismetMathLibrary.RandomFloatInRange` (`self.FMinZ`) (`self.FMaxZ`))))

(fn `UserConstructionScript`)