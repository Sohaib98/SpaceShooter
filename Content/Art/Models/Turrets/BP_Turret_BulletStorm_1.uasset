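; Enemy bullet storm turret that repeatedly fires small enemy projectiles from six spawn points in turn.
; While the shoot flag is set, Tick runs through a short Delay, which throttles the fire rate, then spawns a projectile at the current point.
; An index steps through the spawn array built on BeginPlay and wraps around.
; Projectile Y speed derives from negated actor X scale, so scale affects speed and direction.
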(event `self.ReceiveBeginPlay`
  (`parent.ReceiveBeginPlay`)
  (set `self.ProjectileSpawns` (`|MakeArray` (`self.Projectile1`) (`self.Projectile2`) (`self.Projectile3`) (`self.Projectile4`) (`self.Projectile5`) (`self.Projectile6`))))

(event `self.ReceiveTick`
  (params (DeltaSeconds :type "Float (single-precision)"))
  (bind _iprojectileindex (`self.IProjectileIndex`))
  (bind _returnvalue_x (`KismetMathLibrary.BreakVector` (* (`self.GetActorScale3D`) -1000.0)))
  (if (`self.BShoot`)
    (`KismetSystemLibrary.Delay` 0.2)
    (`|SpawnActorFromClass` "/Game/Blueprints/Projectiles/BP_ProjectileEnemy.BP_ProjectileEnemy_C" (`SceneComponent.K2_GetComponentToWorld` (`|GetArrayItem` (`self.ProjectileSpawns`) (`self.IProjectileIndex`))) "Undefined" "OverrideRootScale" null 0.0 (`KismetMathLibrary.MakeVector` 0.0 _returnvalue_x) (0.25 0.25 0.25))
    (set `self.IProjectileIndex` (+ _iprojectileindex 1))
    (if (>= _iprojectileindex (`KismetArrayLibrary.Array_Length` (`self.ProjectileSpawns`)))
      (set `self.IProjectileIndex` 0))))

(fn `UserConstructionScript`
  (`parent.UserConstructionScript`))