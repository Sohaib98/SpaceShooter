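; Typhoon launcher turret that continuously fires enemy projectiles from nine muzzle points on a rotating launcher.
; A timeline started on BeginPlay restarts whenever it finishes, driving the Launcher's relative roll.
; Tick runs through a short Delay that throttles firing, spawning BP_ProjectileEnemy at each spawn point in round-robin order.
; Projectile speed scales with the turret's X scale, and damage is passed as zero.
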(event `self.ReceiveBeginPlay`
  (set `self.ProjectileSpawns` (`|MakeArray` (`self.Projectile1`) (`self.Projectile2`) (`self.Projectile3`) (`self.Projectile4`) (`self.Projectile5`) (`self.Projectile6`) (`self.Projectile7`) (`self.Projectile8`) (`self.Projectile9`)))
  (bind (_direction _newtrack_0) (`Timeline|Timeline_0_0_0` :!label _label)
    (:`Update`
      (`SceneComponent.K2_SetRelativeRotation` (`self.Launcher`) (`KismetMathLibrary.MakeRotator` (* _newtrack_0 45.0)) false false))
    (:`Finished`
      (goto _label :!via `PlayFromStart`))))

(event `self.ReceiveTick`
  (params (DeltaSeconds :type "Float (single-precision)"))
  (bind _iprojectileindex (`self.IProjectileIndex`))
  (bind _returnvalue_x (`KismetMathLibrary.BreakVector` (* (`self.GetActorScale3D`) 4000.0)))
  (`KismetSystemLibrary.Delay` 0.2)
  (`|SpawnActorFromClass` "/Game/Blueprints/Projectiles/BP_ProjectileEnemy.BP_ProjectileEnemy_C" (`SceneComponent.K2_GetComponentToWorld` (`|GetArrayItem` (`self.ProjectileSpawns`) (`self.IProjectileIndex`))) "Undefined" "OverrideRootScale" null 0.0 (`KismetMathLibrary.MakeVector` 0.0 _returnvalue_x) (0.25 0.25 0.25))
  (set `self.IProjectileIndex` (+ _iprojectileindex 1))
  (if (>= _iprojectileindex (`KismetArrayLibrary.Array_Length` (`self.ProjectileSpawns`)))
    (set `self.IProjectileIndex` 0)))

(fn `UserConstructionScript`
  (`parent.UserConstructionScript`))